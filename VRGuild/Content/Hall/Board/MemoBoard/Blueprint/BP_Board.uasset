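; Memo board actor in the Hall that lets the player create memos and stick them onto the board at a relative position.
; CreateMemo opens a WBP_Memo widget with that position, binds its create-click event and switches to UI-only input.
; StickWidget restores game input, spawns a BP_Memo at the board location plus offset, assigns it the widget and passes it to StickBoard.
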(event `self.CreateMemo`
  (params (relativePosition :type "Vector Structure"))
  (bind _returnvalue (`|CreateWidget` "/Game/Hall/Board/MemoBoard/UI/WBP_Memo.WBP_Memo_C"))
  (`/Game/Hall/Board/MemoBoard/UI/WBP_Memo.SetLocation` _returnvalue relativePosition)
  (add `/Game/Hall/Board/MemoBoard/UI/WBP_Memo.OnClickCreate` _returnvalue (`|CreateDelegate` :!event `StickWidget`))
  (`UserWidget.AddToViewport` _returnvalue 0)
  (`WidgetBlueprintLibrary.SetInputMode_UIOnlyEx` (`GameplayStatics.GetPlayerController` 0) _returnvalue))

(event `StickWidget`
  (params (RelativeLocation :type "Vector Structure") (MemoWidget :type "UserWidget Object Reference"))
  (`WidgetBlueprintLibrary.SetInputMode_GameOnly` (`GameplayStatics.GetPlayerController` 0))
  (bind _returnvalue (`|SpawnActorFromClass` "/Game/Hall/Board/MemoBoard/Blueprint/BP_Memo.BP_Memo_C" (`KismetMathLibrary.Conv_VectorToTransform` (+ RelativeLocation (`self.K2_GetActorLocation`))) "Undefined" "MultiplyWithRoot" null null))
  (`/Game/Hall/Board/MemoBoard/Blueprint/BP_Memo.SetWidget` _returnvalue MemoWidget)
  (`self.StickBoard` _returnvalue RelativeLocation))

(fn `UserConstructionScript`)