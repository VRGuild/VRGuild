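; Player character Blueprint for the Hall that assembles a customizable body from head, body and lower skeletal mesh parts.
; AttachCustomSKMComponents passes its selections to SetupCustomCharacter, which adds the three part components and collects them in CharacterPartBase.
; Each part switches to a hardcoded mesh 1 with a debug index print, leaving the passed selections unapplied.
; Key 1 plays the POINT montage through ACAnimMontage.
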(event `self.AttachCustomSKMComponents`
  (params (customData :type "CharacterCustomData Structure"))
  (`self.SetupCustomCharacter` customData_Selections))

(event `Key|One`
  (params (Key :type "Key Structure"))
  (:`Pressed`
    (`/Game/Character/Player/Animation/montage/AC_AnimMontage.BP_StartAnimMontage` (`self.AC_AnimMontage`) "POINT")))

(fn `SetupCustomCharacter`
  (params (CustomDataSelections :type "Array of Integer"))
  (locals (`Custom Data Selections` :type "Array of Integer") (CharacterPartBase :type "Array of CACCharacterPartBase Object Reference"))
  (set `local.Custom Data Selections` CustomDataSelections)
  (`KismetArrayLibrary.Array_Clear` (`local.CharacterPartBase`))
  (bind _returnvalue (`AddComponent|NODE_AddAC_CustomHead-0`))
  (`KismetArrayLibrary.Array_Add` (`local.CharacterPartBase`) _returnvalue)
  (bind _returnvalue_2 (`AddComponent|NODE_AddAC_CustomBody-0`))
  (`KismetArrayLibrary.Array_Add` (`local.CharacterPartBase`) _returnvalue_2)
  (bind _returnvalue_3 (`AddComponent|NODE_AddAC_CustomLower-0`))
  (`KismetArrayLibrary.Array_Add` (`local.CharacterPartBase`) _returnvalue_3)
  (for (_array_element _array_index) (`local.CharacterPartBase`)
    (`KismetSystemLibrary.PrintString` (`KismetStringLibrary.Conv_IntToString` _array_index))
    (`CACCharacterPartBase.SwitchSKM` _array_element 1)))

(fn `UserConstructionScript`)