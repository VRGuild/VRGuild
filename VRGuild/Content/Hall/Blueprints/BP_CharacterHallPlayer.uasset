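; Player character for the Hall, with modular appearance, a voice-chat indicator and local menus.
; Custom data drives head, body and lower mesh swaps, and sets up the message boards shown over other players.
; On clients, SoundHover shows while the player talks, with the voice synth envelope feeding glow through a material parameter collection.
; ESC info and discard popups switch to UI-only input and flag the player as interacting; key 1 plays a dance montage.
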(event `self.BP_CustomDataUpdate`
  (params (customData :type "CharacterCustomData Structure"))
  (`self.SetupCustomDataUpdate` customData))

(event `Key|One`
  (params (Key :type "Key Structure"))
  (:`Pressed`
    (`/Game/Character/Player/Animation/montage/AC_AnimMontage.BP_StartAnimMontage` (`self.AC_AnimMontage`) "DANCE")))

(event `self.DiscardCarryObject`
  (bind _asplayer_controller (cast `PlayerController` (`self.GetController`) :!pure true))
  (`/Engine/EditorBlueprintResources/StandardMacros.IsValid` (`self.EIKVoiceChatSynth`)
    (:`Is Valid`
      (`KismetSystemLibrary.PrintString` "Voice synth vvalid"))
    (:`Is Not Valid`
      (`KismetSystemLibrary.PrintString` "Voice synth invalid")))
  (bind _returnvalue (`|CreateWidget` "/Game/Character/UI/Popup/WBP_character_popup_throwaway.WBP_character_popup_throwaway_C" _asplayer_controller))
  (`UserWidget.AddToViewport` _returnvalue 0)
  (`WidgetBlueprintLibrary.SetInputMode_UIOnlyEx` _asplayer_controller _returnvalue)
  (set `PlayerController.bShowMouseCursor` true _asplayer_controller)
  (`self.SetInteracting` self true))

(event `self.DisplayESCMenu`
  (bind _returnvalue (`GameplayStatics.GetPlayerController` 0))
  (bind _characterinfowidget (`self.CharacterInfoWidget`))
  (`/Game/Character/UI/MainMenu/WBP_Character_info.SetInfo` _characterinfowidget)
  (`Widget.SetVisibility` _characterinfowidget "Visible")
  (set `PlayerController.bShowMouseCursor` true _returnvalue)
  (`WidgetBlueprintLibrary.SetInputMode_UIOnlyEx` _returnvalue (`self.CharacterInfoWidget`) "DoNotLock" true)
  (`Widget.SetVisibility` (`self.MainUIWidget`) "Hidden")
  (`self.SetInteracting` self true))

(event `ServerSoundhover`
  ;[1 1 1 0.5] Multicast 기능 error 수정 필요
  (`self.MultiSoundhover`))

(event `MultiSoundhover`
  ;[1 1 1 0.5] Multicast 기능 error 수정 필요
)

(event `self.ReceiveBeginPlay`
  (`parent.ReceiveBeginPlay`)
  (`self.SetInteracting` self)
  (`|ExecutionSequence`
    (:`then_0`
      (if (`self.IsLocallyControlled`)
        (bind _asplayer_controller (cast `PlayerController` (`self.GetController`)))
        (bind _returnvalue (`|CreateWidget` "/Game/Character/UI/MainMenu/WBP_Character_info.WBP_Character_info_C" _asplayer_controller (`self.MainUIWidget`)))
        (bind _output_get (set `self.CharacterInfoWidget` _returnvalue))
        (`UserWidget.AddToViewport` _output_get 0)
        (`Widget.SetVisibility` (`self.CharacterInfoWidget`) "Hidden")))
    (:`then_1`
      (`/Engine/EditorBlueprintResources/ActorMacros.Switch Has Authority`
        (:`Remote`
          (bind _returnvalue_2 (`PrimitiveComponent.CreateDynamicMaterialInstance` (`self.SoundHover`) 0 "/Game/Character/UI/Soundhover/M_Sound_Inst.M_Sound_Inst" "None"))
          (`PrimitiveComponent.SetMaterial` (`self.SoundHover`) 1 _returnvalue_2))))))

(event `self.ReceiveTick`
  (params (DeltaSeconds :type "Float (single-precision)"))
  (`parent.ReceiveTick` DeltaSeconds)
  (if (not (`self.HasAuthority`))
    (`|ExecutionSequence`
      (:`then_0`
        ;[1 1 1 0.5] Sound_bool 값으로 변경 필요
        (if (and (`EVIK_Functions.IsPlayerTalking` (`self.GetVoiceChatUserName`)) (> (stale `self.EIKVoiceChatSynth.OnAudioEnvelopeValue` EnvelopeValue) 0.0009))
          (`SceneComponent.SetVisibility` (`self.SoundHover`) true false)
          (`KismetMaterialLibrary.SetScalarParameterValue` "/Game/Character/UI/Soundhover/shinningIndex.shinningIndex" "GlowIntensity" (`self.GlowIntensity`))
          (`PrimitiveComponent.CreateDynamicMaterialInstance` (`self.SoundHover`) 1 "/Game/Character/UI/Soundhover/M_Sound_Inst.M_Sound_Inst" "None")
          (else
            (`SceneComponent.SetVisibility` (`self.SoundHover`) false false))))
      (:`then_1`
        (if (not (`self.IsLocallyControlled`))
          (`/Game/Character/Custom/Blueprints/AC_MsgBoard.Update` (`self.AC_MsgBoard`)))))))

(event `self.EIKVoiceChatSynth.OnAudioEnvelopeValue`
  (params (EnvelopeValue :type "Float (single-precision)"))
  (`KismetSystemLibrary.PrintString` (`KismetStringLibrary.Concat_StrStr` "On Audio Envelop Value: " (`KismetStringLibrary.Conv_DoubleToString` EnvelopeValue) ", Is Playing: " (`KismetStringLibrary.Conv_BoolToString` (`SynthComponent.IsPlaying` (`self.EIKVoiceChatSynth`)))) true false (struct :`R` 0.157069 :`G` 1.0 :`A` 1.0) 0.0)
  (set `self.GlowIntensity` (* EnvelopeValue 200.0)))

(fn `SetupCustomCharacter`
  (params (CustomDataSelections :type "Array of Integer"))
  (locals (`Custom Data Selections` :type "Array of Integer") (CharacterPartBase :type "Array of CACCharacterPartBase Object Reference"))
  (set `local.Custom Data Selections` CustomDataSelections)
  (`KismetArrayLibrary.Array_Clear` (`local.CharacterPartBase`))
  (bind _returnvalue (`AddComponent|NODE_AddAC_CustomHead-0`))
  (`KismetArrayLibrary.Array_Add` (`local.CharacterPartBase`) _returnvalue)
  (bind _returnvalue_2 (`AddComponent|NODE_AddAC_CustomBody-0`))
  (`KismetArrayLibrary.Array_Add` (`local.CharacterPartBase`) _returnvalue_2)
  (bind _returnvalue_3 (`AddComponent|NODE_AddAC_CustomLower-0`))
  (`KismetArrayLibrary.Array_Add` (`local.CharacterPartBase`) _returnvalue_3)
  (for (_array_element _array_index) (`local.CharacterPartBase`)
    (bind _output (`|GetArrayItem` (`local.Custom Data Selections`) _array_index))
    (`KismetSystemLibrary.PrintString` (`KismetStringLibrary.Concat_StrStr` "Data: " (`KismetStringLibrary.Conv_IntToString` _output)) true true (struct :`G` 0.66 :`B` 1.0 :`A` 1.0) 10.0)
    (`CACCharacterPartBase.SwitchSKM` _array_element _output)))

(fn `SetupCustomDataUpdate`
  (params (CustomData :type "CharacterCustomData Structure"))
  (locals (Custom :type "Array of Integer") (Nickname :type String) (Data :type "CharacterCustomData Structure"))
  (set `local.Data` CustomData)
  (`KismetArrayLibrary.Array_Clear` (`local.Custom`))
  (set `local.Custom` (`.Selections` (break `CharacterCustomData` CustomData)))
  (`|ExecutionSequence`
    (:`then_0`
      (`self.SetupCustomCharacter` (`local.Custom`)))
    (:`then_1`
      (if (`self.IsLocallyControlled`)
        (bind _outactors (`GameplayStatics.GetAllActorsOfClass` "BP_CharacterHallPlayer_C"))
        (for _array_element _outactors
          (if (not (== _array_element self))
            (`/Game/Character/Custom/Blueprints/AC_MsgBoard.Init` (`/Game/Hall/Blueprints/BP_CharacterHallPlayer.AC_MsgBoard` _array_element) self)))
        (else
          (`/Game/Character/Custom/Blueprints/AC_MsgBoard.SetHover` (`self.AC_MsgBoard`) (`local.Data`))
          (`KismetSystemLibrary.PrintString` "Not LocallyControlled: Set Hover Custom Data"))))))

(fn `UserConstructionScript`)