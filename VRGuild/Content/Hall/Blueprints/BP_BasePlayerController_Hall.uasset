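; Hall player controller that stores Epic user info in GI_Base, adds a collapsed message board and handles EOS voice chat.
; Voice login chains async callbacks from initialization to joining a hard-coded Team2 room, passing the voice name to the character.
; Tick prints debug talk states and volumes, and key 0 leaves both team rooms.
; Custom character mesh setup and its popup are present but unwired.
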(event `Set User Info`
  (params (UserInfo :type "UserInfo Structure"))
  (bind (_userid _epicaccountid _steamaccountid _characterid _devid _businessid _channellist _experiencevalue _experiencelist _nickname) (break `UserInfo` UserInfo))
  ;[1 1 1] Set Default User Info
  (bind _asgi_base (cast `/Game/Global/GI_Base` (`GameplayStatics.GetGameInstance`)))
  (`|ExecutionSequence`
    (:`then_0`
      (`CGIGameInstance.SetEpicUserIdInstance` _asgi_base (`KismetMathLibrary.Conv_IntToInt64` _userid)))
    (:`then_1`
      (`CGIGameInstance.SetEpicNickNameInstance` _asgi_base _nickname))))

(event `self.OnLoginAPICall`
  ;[1 1 1] Login in Epic
  (`|ExecutionSequence`
    (:`then_0`
      (bind _returnvalue (`AddComponent|NODE_AddAC_UserAPI-0`))
      (add `/Game/Global/API/AC_UserAPI.OnUserOwnInfoGet` _returnvalue (`|CreateDelegate` :!event `Set User Info`))
      (`CACUserAPI.UserOwnInfoGetCall` _returnvalue))))

(event `self.AttachCustomSKMComponents`
  (params (customData :type "CharacterCustomData Structure")))

(event `self.ReceiveBeginPlay`
  (if (`self.IsLocalPlayerController`)
    (bind _returnvalue (`AddComponent|NODE_AddAC_MsgBoard-0` :`self` (`self.K2_GetPawn`)))
    (bind _output_get (set `self.MsgBoard` _returnvalue))
    (bind _widgetmsgboard (`/Game/Character/Custom/Blueprints/AC_MsgBoard.WidgetMsgBoard` _output_get))
    (`/Engine/EditorBlueprintResources/StandardMacros.IsValid` _widgetmsgboard
      (:`Is Valid`
        (`/Game/Character/Message/WBP_MsgBoard.SetVisibleBoard` _widgetmsgboard "Collapsed")))))

(event `self.LoginVoiceChatWithEIK`
  (if (`self.IsLocalPlayerController`)
    (bind _returnvalue (`EVIK_Functions.InitializeEOSVoiceChat`))
    (if _returnvalue
      (`EVIK_Functions.ConnectVoiceChat` (delegate `ConnectToEOSVoiceChat_Result`))
      (else
        (`KismetSystemLibrary.PrintString` "Initialize EOS Voice Chat failed")))))

(event `ConnectToEOSVoiceChat_Result`
  (params (bWasSuccess :type Boolean) (Result :type "EEVIKResultCodes Enum" :default "Success"))
  (if bWasSuccess
    (`EVIK_Functions.LoginEOSVoiceChat` (`EIK_Subsystem.GetProductUserID` (`.ReturnValue` (`EIK_BlueprintFunctions.GetUserUniqueID` self))) (delegate `LoginToEOSVoiceChat_Result`))))

(event `LoginToEOSVoiceChat_Result`
  (params (bWasSuccess :type Boolean) (Result :type "EEVIKResultCodes Enum" :default "Success"))
  (bind _returnvalue (`EVIK_Functions.LoggedInUser`))
  (if bWasSuccess
    (`/Game/TPS/ThirdPerson/Blueprints/BP_ThirdPersonCharacter.ServerSetVoiceChatName` (cast `/Game/TPS/ThirdPerson/Blueprints/BP_ThirdPersonCharacter` (`self.K2_GetPawn`) :!pure true) _returnvalue)
    (`EVIK_Functions.EOSRoomToken` "Team2" _returnvalue "10.0.0.1" (delegate `GetEOSVoiceRoomToken_Result`))))

(event `GetEOSVoiceRoomToken_Result`
  (params (bWasSuccess :type Boolean) (RoomData :type String))
  (if bWasSuccess
    (`KismetSystemLibrary.PrintString` "Voice Room Token Success")
    (else
      (`KismetSystemLibrary.PrintString` "Voice Room Token Failed")))
  (`EVIK_Functions.JoinEOSRoom` "Team2" RoomData false (delegate `JoinEOSVoiceRoom_Result`)))

(event `JoinEOSVoiceRoom_Result`
  (params (bWasSuccess :type Boolean) (Result :type "EEVIKResultCodes Enum" :default "Success"))
  (if bWasSuccess
    (`KismetSystemLibrary.PrintString` "Join EOS Voice Room Success")
    (else
      (`KismetSystemLibrary.PrintString` "Join EOS Voice Room Failed"))))

(event `self.ReceiveTick`
  (params (DeltaSeconds :type "Float (single-precision)"))
  (if (`self.IsLocalPlayerController`)
    (`|ExecutionSequence`
      (:`then_0`
        (bind _returnvalue (`EVIK_Functions.GetAllRooms`))
        (for _array_element _returnvalue
          (`KismetSystemLibrary.PrintString` _array_element true false (struct :`R` 1.0 :`B` 0.104708 :`A` 1.0) 0.0)
          (bind _returnvalue_2 (`EVIK_Functions.GetPlayersInRoom` _array_element))
          (for (_array_element_2 _array_index) _returnvalue_2
            (if (`EVIK_Functions.IsPlayerTalking` _array_element_2)
              (bind _returnvalue_3 (`KismetStringLibrary.Conv_IntToString` _array_index))
              (`KismetSystemLibrary.PrintString` (`KismetStringLibrary.Concat_StrStr` _returnvalue_3 ": " _array_element_2 " Is Speaking") true false (struct :`R` 1.0 :`G` 0.107606 :`A` 1.0) 0.0)
              (else
                (`KismetSystemLibrary.PrintString` (`KismetStringLibrary.Concat_StrStr` _returnvalue_3 ": " _array_element_2 " Is Silent") true false (struct :`G` 1.0 :`B` 0.164013 :`A` 1.0) 0.0))))))
      (:`then_1`
        (bind _outactors (`GameplayStatics.GetAllActorsOfClass` "/Game/TPS/ThirdPerson/Blueprints/BP_ThirdPersonCharacter.BP_ThirdPersonCharacter_C"))
        (for (_array_element_3 _array_index_2) _outactors
          (`self.CheckVoiceChat` _array_element_3 _array_index_2))))))

(event `Key|Zero`
  (params (Key :type "Key Structure"))
  (:`Pressed`
    (`EVIK_Functions.LeaveEOSRoom` "Team1" (delegate `Left`))))

(event `Left`
  (params (bWasSuccess :type Boolean) (Result :type "EEVIKResultCodes Enum" :default "Success"))
  (`KismetSystemLibrary.PrintString` "Left Team 1")
  (`EVIK_Functions.LeaveEOSRoom` "Team2" (delegate `CustomEvent`)))

(event `CustomEvent`
  (params (bWasSuccess :type Boolean) (Result :type "EEVIKResultCodes Enum" :default "Success"))
  (`KismetSystemLibrary.PrintString` "Left Team 2"))

(fn `SetupCustomCharacter`
  (params (CustomDataSelections :type "Array of Integer"))
  (locals (`Custom Data Selections` :type "Array of Integer"))
  (bind _returnvalue (`self.K2_GetPawn`))
  (set `local.Custom Data Selections` CustomDataSelections)
  (`KismetArrayLibrary.Array_Clear` (`self.CharacterPartBase`))
  (bind _returnvalue_2 (`AddComponent|NODE_AddAC_CustomHead-4` :`self` _returnvalue))
  (`KismetArrayLibrary.Array_Add` (`self.CharacterPartBase`) _returnvalue_2)
  (bind _returnvalue_3 (`AddComponent|NODE_AddAC_CustomBody-3` :`self` _returnvalue))
  (`KismetArrayLibrary.Array_Add` (`self.CharacterPartBase`) _returnvalue_3)
  (bind _returnvalue_4 (`AddComponent|NODE_AddAC_CustomLower-3` :`self` _returnvalue))
  (`KismetArrayLibrary.Array_Add` (`self.CharacterPartBase`) _returnvalue_4)
  (for (_array_element _array_index) (`self.CharacterPartBase`)
    (`KismetSystemLibrary.PrintString` (`KismetStringLibrary.Conv_IntToString` _array_index))
    (`CACCharacterPartBase.SwitchSKM` _array_element 1)))

(fn `UserConstructionScript`)