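; BP_BarManager animates a seller NPC in the hall, presumably the bar's keeper, and reacts when the player comes near.
; On BeginPlay it caches the hall player character, then after a delay plays a victory idle and settles into a looping idle.
; When that player enters the Sphere, it plays a happy hand gesture and returns to idle, with the AnimTime flag blocking retriggers until the gesture's delay ends.
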(event `self.ReceiveBeginPlay`
  (`|ExecutionSequence`
    (:`then_0`
      (bind _returnvalue (`GameplayStatics.GetActorOfClass` "/Game/Hall/Blueprints/BP_CharacterHallPlayer.BP_CharacterHallPlayer_C"))
      (set `self.Hall Character` _returnvalue))
    (:`then_1`
      (`KismetSystemLibrary.Delay` 6.0)
      (`SkeletalMeshComponent.PlayAnimation` (`self.SkeletalMesh`) "/Game/NPC/Animation/AN_npc_seller_VictoryIdle_UE.AN_npc_seller_VictoryIdle_UE" false)
      (`KismetSystemLibrary.Delay` 2.0)
      (`SkeletalMeshComponent.PlayAnimation` (`self.SkeletalMesh`) "/Game/Character/NPC/Mesh/NPC_Seller_Animation_Idle_Anim.NPC_Seller_Animation_Idle_Anim" true))))

(event `self.Sphere.OnComponentBeginOverlap`
  (params (OverlappedComponent :type "PrimitiveComponent Object Reference") (OtherActor :type "Actor Object Reference") (OtherComp :type "PrimitiveComponent Object Reference") (OtherBodyIndex :type Integer) (bFromSweep :type Boolean) (SweepResult :type "HitResult Structure (by ref)"))
  (bind _skeletalmesh (`self.SkeletalMesh`))
  (if (== OtherActor (`self.Hall Character`))
    (if (`self.bAnimTime`)
      (`SkeletalMeshComponent.PlayAnimation` _skeletalmesh "/Game/Character/NPC/Animation/AN_NPC_HappyHandGesture_UE.AN_NPC_HappyHandGesture_UE" false)
      (set `self.bAnimTime` false)
      (`KismetSystemLibrary.Delay` 3.0)
      (`SkeletalMeshComponent.PlayAnimation` _skeletalmesh "/Game/Character/NPC/Mesh/NPC_Seller_Animation_Idle_Anim.NPC_Seller_Animation_Idle_Anim" true)
      (set `self.bAnimTime` true))))

(fn `UserConstructionScript`)