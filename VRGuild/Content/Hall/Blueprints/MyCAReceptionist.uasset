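; Receptionist NPC for the Hall that highlights when traced and shows popup widgets to the player.
; Trace begin and end events toggle the visibility of its Outline component.
; Display events add a default NPC template widget or a commission popup to the viewport.
; Only the commission popup is stored and removed on a false Display; the default popup has no removal path.
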(event `self.TraceBegin`
  (`SceneComponent.SetVisibility` (`self.Outline`) true false))

(event `self.TraceEnd`
  (`SceneComponent.SetVisibility` (`self.Outline`) false false))

(event `self.DisplayDefaultPopup`
  (params (bDisplay :type Boolean))
  (if bDisplay
    (bind _returnvalue (`|CreateWidget` "/Game/NPC/UI/WBP_NPC_Templates.WBP_NPC_Templates_C"))
    (`UserWidget.AddToViewport` _returnvalue 0)))

(event `self.DisplayCommossionPopup`
  (params (bDisplay :type Boolean))
  (if bDisplay
    (bind _returnvalue (`|CreateWidget` "/Game/NPC/UI/WBP_npc_popup_project3.WBP_npc_popup_project3_C"))
    (bind _output_get (set `self.WBP_NPC_Commission` _returnvalue))
    (`UserWidget.AddToViewport` _output_get 0)
    (else
      (`Widget.RemoveFromParent` (`self.WBP_NPC_Commission`))
      (set `self.WBP_NPC_Commission` null))))

(fn `UserConstructionScript`)