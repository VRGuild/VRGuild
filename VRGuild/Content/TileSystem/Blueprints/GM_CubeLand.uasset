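; GM_CubeLand is a game mode that builds a furnished CubeLand room with boards, a portal, chairs, tables and NPCs.
; On BeginPlay, the authority spawns an A_TileZone and feeds it a hardcoded square tile grid to create the floor.
; SettingObjects temporarily spawns each prop and NPC class to capture its object info, destroys it, then passes the list with hardcoded placements to the zone's CreateObjectZone.
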(event `CompleteCallApi`
  (params (tileInfo :type "TileInfo Structure (by ref)"))
  ;[1 1 1] Create Room
  (for _index (range -1 4)
    (for _index_2 (range -1 4)
      (`KismetArrayLibrary.Array_Add` (`self.Tile List`) (`KismetMathLibrary.MakeVector_NetQuantize` (`KismetMathLibrary.Conv_IntToDouble` _index) (`KismetMathLibrary.Conv_IntToDouble` _index_2)))))
  (`CATileZone.CreateFloorZone` (`self.TileZone`) (make `TileInfo` (`self.Tile List`)))
  (`self.SettingObjects`))

(event `SettingObjects`
  (bind _board (`self.Board`))
  (bind _returnvalue (`|SpawnActorFromClass` "/Game/TileSystem/Blueprints/Objects/BP_BoardPDF.BP_BoardPDF_C" (`KismetMathLibrary.MakeTransform` (0.0 0.0 0.0)) "Undefined" "MultiplyWithRoot" null null))
  (set `self.Board` _returnvalue)
  (bind _returnvalue_2 (`FL_TileTools.CreateTileObjectInfo` _board))
  (bind (_objectid _objectname _objectclassname) (break `TileObjectInfo` _returnvalue_2))
  (set `self.Array` (`|MakeArray` (make `TileObjectInfo` 0 _objectname _objectclassname (1200.0 1070.0 0.0) (struct :`Yaw` -180.0))))
  (`self.K2_DestroyActor` _board)
  (bind _returnvalue_3 (`|SpawnActorFromClass` "/Game/TileSystem/Blueprints/Objects/BP_BoardProject.BP_BoardProject_C" (`KismetMathLibrary.MakeTransform` (0.0 0.0 0.0)) "Undefined" "MultiplyWithRoot" null null))
  (set `self.BoardWide` _returnvalue_3)
  (bind _returnvalue_4 (`FL_TileTools.CreateTileObjectInfo` (`self.BoardWide`)))
  (bind (_objectid_2 _objectname_2 _objectclassname_2) (break `TileObjectInfo` _returnvalue_4))
  (`KismetArrayLibrary.Array_Add` (`self.Array`) (make `TileObjectInfo` 0 _objectname_2 _objectclassname_2 (400.0 -500.0 0.0) (struct :`Yaw` 90.0)))
  (`self.K2_DestroyActor` (`self.BoardWide`))
  (bind _returnvalue_5 (`|SpawnActorFromClass` "/Game/TileSystem/Blueprints/Objects/BP_Potal.BP_Potal_C" (`KismetMathLibrary.MakeTransform` (0.0 0.0 0.0)) "Undefined" "MultiplyWithRoot" null null))
  (bind _output_get (set `self.Potal` _returnvalue_5))
  (bind _returnvalue_6 (`FL_TileTools.CreateTileObjectInfo` _output_get))
  (bind (_objectid_3 _objectname_3 _objectclassname_3) (break `TileObjectInfo` _returnvalue_6))
  (`KismetArrayLibrary.Array_Add` (`self.Array`) (make `TileObjectInfo` 0 _objectname_3 _objectclassname_3 (-300.0 1120.0 0.0) (struct :`Yaw` 45.0)))
  (`self.K2_DestroyActor` _returnvalue_5)
  (bind _returnvalue_7 (`|SpawnActorFromClass` "/Game/Hall/Board/MemoBoard/Blueprint/BP_Board.BP_Board_C" (`KismetMathLibrary.MakeTransform` (0.0 0.0 0.0)) "Undefined" "MultiplyWithRoot" null null))
  (bind _returnvalue_8 (`FL_TileTools.CreateTileObjectInfo` _returnvalue_7))
  (bind (_objectid_4 _objectname_4 _objectclassname_4) (break `TileObjectInfo` _returnvalue_8))
  (`KismetArrayLibrary.Array_Add` (`self.Array`) (make `TileObjectInfo` 0 _objectname_4 _objectclassname_4 (1200.0 240.0 0.0) (struct :`Yaw` 180.0)))
  (`self.K2_DestroyActor` _returnvalue_7)
  (bind _returnvalue_9 (`|SpawnActorFromClass` "/Game/TileSystem/Blueprints/Objects/BP_Chair.BP_Chair_C" (`KismetMathLibrary.MakeTransform` (0.0 0.0 0.0)) "Undefined" "MultiplyWithRoot" null null))
  (bind _returnvalue_10 (`FL_TileTools.CreateTileObjectInfo` _returnvalue_9))
  (bind (_objectid_5 _objectname_5 _objectclassname_5) (break `TileObjectInfo` _returnvalue_10))
  (`KismetArrayLibrary.Array_Add` (`self.Array`) (make `TileObjectInfo` 0 _objectname_5 _objectclassname_5 (180.0 60.0 0.0) (struct :`Yaw` -90.0)))
  (`self.K2_DestroyActor` _returnvalue_9)
  (bind _returnvalue_11 (`|SpawnActorFromClass` "/Game/TileSystem/Blueprints/Objects/BP_Chair.BP_Chair_C" (`KismetMathLibrary.MakeTransform` (0.0 0.0 0.0)) "Undefined" "MultiplyWithRoot" null null))
  (bind _returnvalue_12 (`FL_TileTools.CreateTileObjectInfo` _returnvalue_11))
  (bind (_objectid_6 _objectname_6 _objectclassname_6) (break `TileObjectInfo` _returnvalue_12))
  (`KismetArrayLibrary.Array_Add` (`self.Array`) (make `TileObjectInfo` 0 _objectname_6 _objectclassname_6 (460.0 60.0 0.0) (struct :`Yaw` 90.0)))
  (`self.K2_DestroyActor` _returnvalue_11)
  (bind _returnvalue_13 (`|SpawnActorFromClass` "/Game/TileSystem/Blueprints/Objects/Sitting_chair_Child.Sitting_chair_Child_C" (`KismetMathLibrary.MakeTransform` (0.0 0.0 0.0)) "Undefined" "MultiplyWithRoot" null null))
  (bind _returnvalue_14 (`FL_TileTools.CreateTileObjectInfo` _returnvalue_13))
  (bind (_objectid_7 _objectname_7 _objectclassname_7) (break `TileObjectInfo` _returnvalue_14))
  (`KismetArrayLibrary.Array_Add` (`self.Array`) (make `TileObjectInfo` 0 _objectname_7 _objectclassname_7 (180.0 330.0 0.0) (struct :`Yaw` -90.0)))
  (`self.K2_DestroyActor` _returnvalue_13)
  (bind _returnvalue_15 (`|SpawnActorFromClass` "/Game/TileSystem/Blueprints/Objects/Sitting_chair_Child.Sitting_chair_Child_C" (`KismetMathLibrary.MakeTransform` (0.0 0.0 0.0)) "Undefined" "MultiplyWithRoot" null null))
  (bind _returnvalue_16 (`FL_TileTools.CreateTileObjectInfo` _returnvalue_15))
  (bind (_objectid_8 _objectname_8 _objectclassname_8) (break `TileObjectInfo` _returnvalue_16))
  (`KismetArrayLibrary.Array_Add` (`self.Array`) (make `TileObjectInfo` 0 _objectname_8 _objectclassname_8 (460.0 330.0 0.0) (struct :`Yaw` 90.0)))
  (`self.K2_DestroyActor` _returnvalue_15)
  (bind _returnvalue_17 (`|SpawnActorFromClass` "/Game/TileSystem/Blueprints/Objects/BP_Table.BP_Table_C" (`KismetMathLibrary.MakeTransform` (0.0 0.0 0.0)) "Undefined" "MultiplyWithRoot" null null))
  (bind _returnvalue_18 (`FL_TileTools.CreateTileObjectInfo` _returnvalue_17))
  (bind (_objectid_9 _objectname_9 _objectclassname_9) (break `TileObjectInfo` _returnvalue_18))
  (`KismetArrayLibrary.Array_Add` (`self.Array`) (make `TileObjectInfo` 0 _objectname_9 _objectclassname_9 (330.0 60.0 0.0) (struct :`Yaw` 90.0)))
  (`self.K2_DestroyActor` _returnvalue_17)
  (bind _returnvalue_19 (`|SpawnActorFromClass` "/Game/TileSystem/Blueprints/Objects/BP_Table.BP_Table_C" (`KismetMathLibrary.MakeTransform` (0.0 0.0 0.0)) "Undefined" "MultiplyWithRoot" null null))
  (bind _returnvalue_20 (`FL_TileTools.CreateTileObjectInfo` _returnvalue_19))
  (bind (_objectid_10 _objectname_10 _objectclassname_10) (break `TileObjectInfo` _returnvalue_20))
  (`KismetArrayLibrary.Array_Add` (`self.Array`) (make `TileObjectInfo` 0 _objectname_10 _objectclassname_10 (330.0 330.0 0.0) (struct :`Yaw` 90.0)))
  (`self.K2_DestroyActor` _returnvalue_19)
  (bind _returnvalue_21 (`|SpawnActorFromClass` "/Game/NPC/Blueprints/BP_NpcPlayer10.BP_NpcPlayer10_C" (`KismetMathLibrary.MakeTransform` (0.0 0.0 0.0)) "Undefined" "MultiplyWithRoot" null null))
  (bind _returnvalue_22 (`FL_TileTools.CreateTileObjectInfo` _returnvalue_21))
  (bind (_objectid_11 _objectname_11 _objectclassname_11) (break `TileObjectInfo` _returnvalue_22))
  (`KismetArrayLibrary.Array_Add` (`self.Array`) (make `TileObjectInfo` 0 _objectname_11 _objectclassname_11 (1000.0 1100.0 10.0) (struct :`Yaw` 230.0)))
  (`/Engine/EditorBlueprintResources/StandardMacros.IsValid` _returnvalue_21
    (:`Is Valid`
      (`self.K2_DestroyActor` _returnvalue_21))
    (:`Is Not Valid`
      _))
  (bind _returnvalue_23 (`|SpawnActorFromClass` "/Game/NPC/Blueprints/BP_NpcPlayer16.BP_NpcPlayer16_C" (`KismetMathLibrary.MakeTransform` (0.0 0.0 0.0)) "Undefined" "MultiplyWithRoot" null null))
  (bind _returnvalue_24 (`FL_TileTools.CreateTileObjectInfo` _returnvalue_23))
  (bind (_objectid_12 _objectname_12 _objectclassname_12) (break `TileObjectInfo` _returnvalue_24))
  (`KismetArrayLibrary.Array_Add` (`self.Array`) (make `TileObjectInfo` 0 _objectname_12 _objectclassname_12 (-65.0 -380.0 90.0) (struct :`Yaw` -60.0)))
  (`/Engine/EditorBlueprintResources/StandardMacros.IsValid` _returnvalue_23
    (:`Is Valid`
      (`self.K2_DestroyActor` _returnvalue_23))
    (:`Is Not Valid`
      _))
  (bind _returnvalue_25 (`|SpawnActorFromClass` "/Game/NPC/Blueprints/BP_NpcPlayer2.BP_NpcPlayer2_C" (`KismetMathLibrary.MakeTransform` (0.0 0.0 0.0)) "Undefined" "MultiplyWithRoot" null null))
  (bind _returnvalue_26 (`FL_TileTools.CreateTileObjectInfo` _returnvalue_25))
  (bind (_objectid_13 _objectname_13 _objectclassname_13) (break `TileObjectInfo` _returnvalue_26))
  (`KismetArrayLibrary.Array_Add` (`self.Array`) (make `TileObjectInfo` 0 _objectname_13 _objectclassname_13 (170.0 70.0 100.0) (struct :`Pitch` 10.0)))
  (`/Engine/EditorBlueprintResources/StandardMacros.IsValid` _returnvalue_25
    (:`Is Valid`
      (`self.K2_DestroyActor` _returnvalue_25))
    (:`Is Not Valid`
      _))
  (bind _returnvalue_27 (`|SpawnActorFromClass` "/Game/NPC/Blueprints/BP_NpcPlayer1.BP_NpcPlayer1_C" (`KismetMathLibrary.MakeTransform` (0.0 0.0 0.0)) "Undefined" "MultiplyWithRoot" null null))
  (bind _returnvalue_28 (`FL_TileTools.CreateTileObjectInfo` _returnvalue_27))
  (bind (_objectid_14 _objectname_14 _objectclassname_14) (break `TileObjectInfo` _returnvalue_28))
  (`KismetArrayLibrary.Array_Add` (`self.Array`) (make `TileObjectInfo` 0 _objectname_14 _objectclassname_14 (430.0 70.0 100.0) (struct :`Yaw` 180.0)))
  (`/Engine/EditorBlueprintResources/StandardMacros.IsValid` _returnvalue_27
    (:`Is Valid`
      (`self.K2_DestroyActor` _returnvalue_27))
    (:`Is Not Valid`
      _))
  (`CATileZone.CreateObjectZone` (`self.TileZone`) (make `TileInfo` :`objectInfoList` (`self.Array`))))

(event `self.ReceiveBeginPlay`
  (`/Engine/EditorBlueprintResources/ActorMacros.Switch Has Authority`
    (:`Authority`
      ;[1 1 1] Tile Create
      (bind _returnvalue (`|SpawnActorFromClass` "/Game/TileSystem/Blueprints/Tiles/A_TileZone.A_TileZone_C" (`KismetMathLibrary.MakeTransform` (0.0 0.0 0.0)) "Undefined" "MultiplyWithRoot" null null))
      (bind _output_get (set `self.TileZone` _returnvalue))
      (set `CATileZone.SpaceType` "Floor" _output_get)
      (`self.CompleteCallApi` (struct)))))

(fn `ObjectSetting`)

(fn `UserConstructionScript`)