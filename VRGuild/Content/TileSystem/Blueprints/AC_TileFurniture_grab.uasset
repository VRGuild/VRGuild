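; Furniture grab component that lets the player carry physics objects with the right mouse button, using the third-person character's PhysicsHandle.
; BeginPlay caches the character by casting the player pawn's owner.
; Pressing traces from FollowCamera on Visibility and grabs the hit component without checking for a hit; releasing drops it.
; While grabbing, Tick moves the handle target a fixed distance ahead of the camera and prints debug text.
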(event `self.ReceiveBeginPlay`
  (bind _asbp_third_person_character (cast `/Game/TPS/ThirdPerson/Blueprints/BP_ThirdPersonCharacter` (`Actor.GetOwner` (`GameplayStatics.GetPlayerPawn` 0))))
  (set `self.OwnerCharacter` _asbp_third_person_character))

(event `self.ReceiveTick`
  (params (DeltaSeconds :type "Float (single-precision)"))
  (bind _followcamera (`TP_ThirdPersonCharacter.FollowCamera` (`self.OwnerCharacter`)))
  (if (`self.IsGrabbing`)
    (`KismetSystemLibrary.PrintString` "Hello")
    (`PhysicsHandleComponent.SetTargetLocation` (`/Game/TPS/ThirdPerson/Blueprints/BP_ThirdPersonCharacter.PhysicsHandle` (`self.OwnerCharacter`)) (+ (`SceneComponent.K2_GetComponentLocation` _followcamera) (* (`KismetMathLibrary.GetForwardVector` (`SceneComponent.K2_GetComponentRotation` _followcamera)) 500.0)))))

(event `Key|RightMouseButton`
  (params (Key :type "Key Structure"))
  (bind _followcamera (`TP_ThirdPersonCharacter.FollowCamera` (`self.OwnerCharacter`)))
  (bind _returnvalue (`SceneComponent.K2_GetComponentLocation` _followcamera))
  (:`Pressed`
    (bind _outhit (`KismetSystemLibrary.LineTraceSingle` _returnvalue (+ _returnvalue (* (`KismetMathLibrary.GetForwardVector` (`SceneComponent.K2_GetComponentRotation` _followcamera)) 500.0)) "TraceTypeQuery1"))
    (if true
      (bind (_bblockinghit _binitialoverlap _time _distance _location _impactpoint _normal _impactnormal _physmat _hitactor _hitcomponent) (`GameplayStatics.BreakHitResult` _outhit))
      (`PhysicsHandleComponent.GrabComponentAtLocationWithRotation` :`self` (`/Game/TPS/ThirdPerson/Blueprints/BP_ThirdPersonCharacter.PhysicsHandle` (`self.OwnerCharacter`)) :`Component` _hitcomponent :`Location` (`SceneComponent.K2_GetComponentLocation` _hitcomponent))
      (set `self.IsGrabbing` true)))
  (:`Released`
    (if (`self.IsGrabbing`)
      (`PhysicsHandleComponent.ReleaseComponent` (`/Game/TPS/ThirdPerson/Blueprints/BP_ThirdPersonCharacter.PhysicsHandle` (`self.OwnerCharacter`)))
      (set `self.IsGrabbing` false))))