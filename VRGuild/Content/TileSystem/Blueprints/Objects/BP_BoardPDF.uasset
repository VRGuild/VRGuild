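; Board actor in the tile system that displays a row of PDF documents from a list of URLs.
; On BeginPlay the authority loads a hardcoded two-URL list, spawning one PDF_Actor per URL.
; Each is attached to PositionBase, scaled to half size, spaced along Y by index and given its URL.
; Spawned actors are tracked in PdfList and destroyed along with the board.
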(event `self.ReceiveBeginPlay`
  (`/Engine/EditorBlueprintResources/ActorMacros.Switch Has Authority`
    (:`Authority`
      (`self.LoadPDF` (make `TilePdfInfoList` (`|MakeArray` "https://bitcoin.org/bitcoin.pdf" "http://kocw-n.xcache.kinxcdn.com/data/document/2022/edu/gcu/seokkwangho1216/06-1.pdf"))))))

(event `LoadPDF`
  (params (PDFInfoList :type "TilePdfInfoList Structure"))
  (`KismetArrayLibrary.Array_Clear` (`self.PdfList`))
  (for (_array_element _array_index) (`.pdfUrlList` (break `TilePdfInfoList` PDFInfoList))
    (`self.PostPdf` _array_element _array_index)))

(event `PostPdf`
  (params (TilePDFUrl :type "String (by ref)") (Index :type Integer))
  (bind _returnvalue (`|SpawnActorFromClass` "/Game/Global/PDF/BluePrint/PDF_Actor.PDF_Actor_C" (`KismetMathLibrary.Conv_VectorToTransform` (0.0 0.0 0.0)) "Undefined" "MultiplyWithRoot" null null))
  (`KismetArrayLibrary.Array_Add` (`self.PdfList`) _returnvalue)
  (`|ExecutionSequence`
    (:`then_0`
      (`self.K2_AttachToComponent` _returnvalue (`self.PositionBase`) "None" "KeepRelative" "KeepRelative" "KeepRelative" true)
      (bind _rootcomponent (`Actor.RootComponent` _returnvalue))
      (`SceneComponent.K2_SetRelativeLocation` _rootcomponent (`KismetMathLibrary.MakeVector_NetQuantize` 0.0 (* (`KismetMathLibrary.Conv_IntToDouble` Index) 140.0)) false false)
      (`SceneComponent.SetRelativeScale3D` _rootcomponent (0.5 0.5 0.5)))
    (:`then_1`
      (`/Game/Global/PDF/BluePrint/PDF_Actor.SetInitPdfUrl` _returnvalue TilePDFUrl))))

(event `self.ReceiveDestroyed`
  (for _array_element (`self.PdfList`)
    (`self.K2_DestroyActor` _array_element)))

(fn `UserConstructionScript`)