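; Chair actor that detects when the hall player character is close enough to sit on it.
; Overlap events on SitCollision set the CanSit flag and show or hide the Outline component as a highlight for BP_CharacterHallPlayer only.
; Input from player controller 0 is enabled on BeginPlay, but the graph contains no input handler or sit action.
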(event `self.ReceiveBeginPlay`
  (`self.EnableInput` (`GameplayStatics.GetPlayerController` 0)))

(event `self.Sit Collision.OnComponentBeginOverlap`
  (params (OverlappedComponent :type "PrimitiveComponent Object Reference") (OtherActor :type "Actor Object Reference") (OtherComp :type "PrimitiveComponent Object Reference") (OtherBodyIndex :type Integer) (bFromSweep :type Boolean) (SweepResult :type "HitResult Structure (by ref)"))
  (cast `/Game/Hall/Blueprints/BP_CharacterHallPlayer` OtherActor)
  (set `self.CanSit` true)
  (`SceneComponent.SetVisibility` (`self.Outline`) true false))

(event `self.Sit Collision.OnComponentEndOverlap`
  (params (OverlappedComponent :type "PrimitiveComponent Object Reference") (OtherActor :type "Actor Object Reference") (OtherComp :type "PrimitiveComponent Object Reference") (OtherBodyIndex :type Integer))
  (cast `/Game/Hall/Blueprints/BP_CharacterHallPlayer` OtherActor)
  (set `self.CanSit` false)
  (`SceneComponent.SetVisibility` (`self.Outline`) false false))

(fn `UserConstructionScript`)