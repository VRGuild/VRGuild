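; Player controller for the CubeLand tile space that builds the room and stores user ID and nickname from the user API in the game instance.
; On authority, it spawns a tile zone, lays a square floor grid and places boards and a portal, using short-lived actors to derive their object info.
; On remote, it adds tile interaction with a test default cube.
; Enter travels to the next server.
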(event `Set User Info`
  (params (UserInfo :type "UserInfo Structure"))
  (bind (_userid _epicaccountid _steamaccountid _characterid _devid _businessid _channellist _experiencevalue _experiencelist _nickname) (break `UserInfo` UserInfo))
  ;[1 1 1] User Id
  (bind _asgi_base (cast `/Game/Global/GI_Base` (`GameplayStatics.GetGameInstance`)))
  (`|ExecutionSequence`
    (:`then_0`
      (`CGIGameInstance.SetEpicUserIdInstance` _asgi_base (`KismetMathLibrary.Conv_IntToInt64` (`KismetMathLibrary.Conv_Int64ToInt` _userid))))
    (:`then_1`
      (`CGIGameInstance.SetEpicNickNameInstance` _asgi_base _nickname))))

(event `self.OnLoginAPICall`
  ;[1 1 1] User Id
  (bind _returnvalue (`AddComponent|NODE_AddAC_UserAPI-0`))
  (add `/Game/Global/API/AC_UserAPI.OnUserOwnInfoGet` _returnvalue (`|CreateDelegate` :!event `Set User Info`))
  (`CACUserAPI.UserOwnInfoGetCall` _returnvalue))

(event `ObjectSetting`
  (bind _board (`self.Board`))
  (bind _boardwide (`self.BoardWide`))
  (bind _returnvalue (`|SpawnActorFromClass` "/Game/TileSystem/Blueprints/Objects/BP_BoardPDF.BP_BoardPDF_C" (`KismetMathLibrary.MakeTransform` (0.0 0.0 0.0)) "Undefined" "MultiplyWithRoot" null null))
  (set `self.Board` _returnvalue)
  (bind _returnvalue_2 (`FL_TileTools.CreateTileObjectInfo` _board))
  (bind (_objectid _objectname _objectclassname) (break `TileObjectInfo` _returnvalue_2))
  (bind (_objectid_2 _objectname_2 _objectclassname_2) (break `TileObjectInfo` _returnvalue_2))
  (set `self.Array` (`|MakeArray` (make `TileObjectInfo` 0 _objectname _objectclassname (1200.0 1070.0 0.0)) (make `TileObjectInfo` 0 _objectname_2 _objectclassname_2 (1200.0 -230.0 0.0))))
  (`self.K2_DestroyActor` _board)
  (bind _returnvalue_3 (`|SpawnActorFromClass` "/Game/TileSystem/Blueprints/Objects/BP_BoardProject.BP_BoardProject_C" (`KismetMathLibrary.MakeTransform` (0.0 0.0 0.0)) "Undefined" "MultiplyWithRoot" null null))
  (set `self.BoardWide` _returnvalue_3)
  (bind _returnvalue_4 (`FL_TileTools.CreateTileObjectInfo` _boardwide))
  (bind (_objectid_3 _objectname_3 _objectclassname_3) (break `TileObjectInfo` _returnvalue_4))
  (`KismetArrayLibrary.Array_Add` (`self.Array`) (make `TileObjectInfo` 0 _objectname_3 _objectclassname_3 (530.0 -450.0 0.0) (struct :`Yaw` 90.0)))
  (`self.K2_DestroyActor` _boardwide)
  (bind _returnvalue_5 (`|SpawnActorFromClass` "/Game/TileSystem/Blueprints/Objects/BP_Potal.BP_Potal_C" (`KismetMathLibrary.MakeTransform` (0.0 0.0 0.0)) "Undefined" "MultiplyWithRoot" null null))
  (bind _output_get (set `self.Potal` _returnvalue_5))
  (bind _returnvalue_6 (`FL_TileTools.CreateTileObjectInfo` _output_get))
  (bind (_objectid_4 _objectname_4 _objectclassname_4) (break `TileObjectInfo` _returnvalue_6))
  (`KismetArrayLibrary.Array_Add` (`self.Array`) (make `TileObjectInfo` 0 _objectname_4 _objectclassname_4 (-300.0 1120.0 0.0) (struct :`Yaw` 45.0)))
  (`CATileZone.CreateObjectZone` (`self.TileZone`) (make `TileInfo` :`objectInfoList` (`self.Array`))))

(event `CompleteCallApi`
  (params (tileInfo :type "TileInfo Structure (by ref)"))
  ;[1 1 1] Create Room
  (for _index (range -1 4)
    (for _index_2 (range -1 4)
      (`KismetArrayLibrary.Array_Add` (`self.Tile List`) (`KismetMathLibrary.MakeVector_NetQuantize` (`KismetMathLibrary.Conv_IntToDouble` _index) (`KismetMathLibrary.Conv_IntToDouble` _index_2)))))
  (`CATileZone.CreateFloorZone` (`self.TileZone`) (make `TileInfo` (`self.Tile List`)))
  (`self.ObjectSetting`))

(event `self.ReceiveBeginPlay`
  (`/Engine/EditorBlueprintResources/ActorMacros.Switch Has Authority`
    (:`Authority`
      ;[1 1 1] Tile Create
      (bind _returnvalue (`|SpawnActorFromClass` "/Game/TileSystem/Blueprints/Tiles/A_TileZone.A_TileZone_C" (`KismetMathLibrary.MakeTransform` (0.0 0.0 0.0)) "Undefined" "MultiplyWithRoot" null null))
      (bind _output_get (set `self.TileZone` _returnvalue))
      (set `CATileZone.SpaceType` "Floor" _output_get)
      (`self.CompleteCallApi` (struct)))
    (:`Remote`
      (bind _returnvalue_2 (`AddComponent|NODE_AddAC_TileInteraction-0` :`self` (`GameplayStatics.GetPlayerPawn` 0)))
      ;[1 1 1] 기본 선택 된 오브젝트
      (`CACTileInteraction.SetSelectedTileCube` _returnvalue_2 "/Game/TileSystem/Blueprints/TileCube/A_TileCubeTable_TEST.A_TileCubeTable_TEST_C")
      (`KismetSystemLibrary.Delay` 0.2)
      (`/Engine/EditorBlueprintResources/StandardMacros.IsValid` (`self.K2_GetPawn`)
        (:`Is Valid`
          (`TP_ThirdPersonCharacter.SetInteracting` (cast `TP_ThirdPersonCharacter` (`self.K2_GetPawn`) :!pure true) (`self.K2_GetPawn`) false))))))

(event `Key|Enter`
  (params (Key :type "Key Structure"))
  (:`Pressed`
    (`self.TravelToNextServer`)))

(fn `UserConstructionScript`)