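; AC_TileInteraction handles the purchase step for adding a tile, gated by a cost prompt.
; CheckPayEther opens a WBP_TileCost widget initialized with the price and binds its success and failure events, leaving ItemName unused.
; An IsWaiting flag rejects new requests while a prompt is pending.
; Success clears the flag and calls AddTile, while failure only clears the flag.
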(event `SuccesedBuyTile`
  (set `self.IsWaiting` false)
  (`self.AddTile`))

(event `FailBillTile`
  (set `self.IsWaiting` false))

(fn `CheckPayEther`
  (params (price :type "Ether Structure (by ref)") (itemName :type String))
  (returns (ReturnValue :type Boolean))
  (if (`self.IsWaiting`)
    (return false)
    (else
      (set `self.IsWaiting` true)
      (bind _returnvalue (`|CreateWidget` "/Game/TileSystem/UI/WBP_TileCost.WBP_TileCost_C"))
      (add `/Game/TileSystem/UI/WBP_TileCost.OnSuccessedBuy` _returnvalue (`|CreateDelegate` :!event `SuccesedBuyTile`))
      (add `/Game/TileSystem/UI/WBP_TileCost.OnFaildBill` _returnvalue (`|CreateDelegate` :!event `FailBillTile`))
      (`/Game/TileSystem/UI/WBP_TileCost.SetInit` _returnvalue price)
      (`UserWidget.AddToViewport` _returnvalue 0)
      (return true))))