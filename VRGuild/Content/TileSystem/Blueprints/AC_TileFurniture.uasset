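; AC_TileFurniture is an actor component that lets its owner pick and spawn tile furniture.
; The C key toggles a placement mode, creating or removing the WBP_TileFurniture selection widget.
; In that mode, the mouse wheel steps a clamped selection index and highlights the matching widget button.
; Middle click looks up the selection in TileFurnitureBox and spawns that actor at a fixed world-space offset from the owner.
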(event `self.ReceiveBeginPlay`)

(event `Key|C`
  (params (Key :type "Key Structure"))
  ;[1 1 1 0.5] Furniture select widget create
  (:`Pressed`
    (if (`self.bSpawnFurniture`)
      (set `self.bSpawnFurniture` false)
      (`Widget.RemoveFromParent` (`self.FurnitureUI`))
      (else
        (set `self.bSpawnFurniture` true)
        (bind _returnvalue (`|CreateWidget` "/Game/TileSystem/UI/WBP_TileFurniture.WBP_TileFurniture_C"))
        (bind _output_get (set `self.FurnitureUI` _returnvalue))
        (`UserWidget.AddToViewport` _output_get 0)))))

(event `Key|MouseScrollDown`
  (params (Key :type "Key Structure"))
  ;[1 1 1 0.5] Mouse Wheel Input
  (:`Pressed`
    (if (`self.bSpawnFurniture`)
      (if (not (== (`self.CurrentSpell`) (`/Game/TileSystem/UI/WBP_TileFurniture.ButtonLastSpell` (`self.FurnitureUI`))))
        (bind _output_get (set `self.CurrentSpell` (+ (`self.CurrentSpell`) 1)))
        (`/Game/TileSystem/UI/WBP_TileFurniture.ButtonSelected` (`self.furnitureUI`) _output_get)))))

(event `Key|MouseScrollUp`
  (params (Key :type "Key Structure"))
  ;[1 1 1 0.5] Mouse Wheel Input
  (:`Pressed`
    (if (`self.bSpawnFurniture`)
      (if (not (== (`self.CurrentSpell`) (`self.FirstSpell`)))
        (bind _output_get (set `self.CurrentSpell` (- (`self.CurrentSpell`) 1)))
        (`/Game/TileSystem/UI/WBP_TileFurniture.ButtonSelected` (`self.furnitureUI`) _output_get)))))

(event `Key|MiddleMouseButton`
  (params (Key :type "Key Structure"))
  (bind (_returnvalue_location _returnvalue_rotation _returnvalue_scale) (`KismetMathLibrary.BreakTransform` (`Actor.GetTransform` (`self.GetOwner`))))
  (:`Pressed`
    (if (`self.bSpawnFurniture`)
      ;[1 1 1 0.5] actor와 연계해서 작동할 함수 넣어주면 됨
      (`|SpawnActorFromClass` (break `TileFurnitureInfo` (`BlueprintMapLibrary.Map_Find` (`self.TileFurnitureBox`) (- (`self.CurrentSpell`) 1))) (`KismetMathLibrary.MakeTransform` (- _returnvalue_location (-120.0 0.0 90.0)) _returnvalue_rotation _returnvalue_scale) "Undefined" "MultiplyWithRoot" null null))))