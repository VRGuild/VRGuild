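; PDF display actor that shows document pages on a mesh in the world.
; It loads a PDF from a path or URL, then creates a dynamic M_PDF material on FrontSide and shows the first page.
; SetCurrentPage renders pages asynchronously into that material's texture parameter, driven by next/previous events.
; AutoPaging re-calls itself on a delay to loop pages, skipping the last, but nothing here starts it.
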(event `self.ReceiveBeginPlay`)

(event `AutoPaging`
  (`KismetSystemLibrary.Delay` 3.0)
  (`/Engine/EditorBlueprintResources/StandardMacros.IsValid` (`self.PDFDocument`)
    (:`Is Valid`
      (if (`self.bAutoPage`)
        (`self.Set Current Page` (mod (+ (`self.CurrentPage`) 1) (- (`PDFDocument.GetPageCount` (`self.PDFDocument`)) 1)))
        (`self.AutoPaging`)))))

(event `SetInitPDF`
  (params (Path :type String))
  ;[1 1 1] PDF Load
  (bind (_pdfdocument _errorcode _errormessage) (`LoadPDFDocumentProxy.LoadDocument` Path)
    (:`Loaded`
      (set `self.PDFDocument` _pdfdocument)
      (bind _returnvalue (`PrimitiveComponent.CreateDynamicMaterialInstance` (`self.FrontSide`) 0 "/Game/Global/PDF/Metrial/M_PDF.M_PDF" "None"))
      (set `self.MaterialInstance` _returnvalue)
      (`self.Set Current Page` 0)
      (set `self.bAutoPage` true))
    (:`Error`
      (`KismetSystemLibrary.PrintString` _errormessage))))

(event `SetInitPdfUrl`
  (params (URL :type String))
  (bind _pdfdocument (`LoadPDFDocumentProxy.LoadDocumentFromURL` URL)
    (:`Loaded`
      (set `self.PDFDocument` _pdfdocument)
      (bind _returnvalue (`PrimitiveComponent.CreateDynamicMaterialInstance` (`self.FrontSide`) 0 "/Game/Global/PDF/Metrial/M_PDF.M_PDF" "None"))
      (set `self.MaterialInstance` _returnvalue)
      (`self.Set Current Page` 0)
      (set `self.bAutoPage` true))
    (:`Error`
      (`KismetSystemLibrary.PrintString` "Hello"))))

(event `Set Current Page`
  (params (Index :type Integer))
  (bind _returnvalue (`PDFDocument.GetPage` (`self.PDFDocument`) Index))
  ;[1 1 1] PDF View
  (`/Engine/EditorBlueprintResources/StandardMacros.IsValid` _returnvalue
    (:`Is Valid`
      (set `self.CurrentPage` Index)
      (bind _texture (`RenderPDFPageProxy.RenderPage` _returnvalue (struct) (make `PDFVector2D` (`KismetMathLibrary.FTrunc` (`PDFPage.GetWidth` _returnvalue)) (`KismetMathLibrary.FTrunc` (`PDFPage.GetHeight` _returnvalue))) (struct :`R` 1.0 :`G` 1.0 :`B` 1.0 :`A` 1.0) "Normal")
        (:`Rendered`
          (`MaterialInstanceDynamic.SetTextureParameterValue` (`self.MaterialInstance`) "PDF_Texture" _texture))))))

(event `Previous Page`
  ;[1 1 1] Page System
  (`self.Set Current Page` (+ (`self.CurrentPage`) -1)))

(event `Next Page`
  ;[1 1 1] Page System
  (`self.Set Current Page` (+ (`self.CurrentPage`) 1)))

(event `self.NextCall`
  (`self.Next Page`))

(event `self.PrevCall`
  (`self.Previous Page`))

(fn `OnRep_PDFDocument`)

(fn `UserConstructionScript`)