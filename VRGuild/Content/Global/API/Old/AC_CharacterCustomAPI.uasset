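; AC_CharacterCustomAPI relays results of character customization API calls for get, create, update and delete operations, and sits in an Old API folder.
; Each operation has a success and a failure callback event that fires a matching event dispatcher for listeners.
; Only get and create successes forward parsed data; the event graph contains no request or parsing logic.
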(event `self.OnCharacterCustomGetCallBack`
  (params (ParseData :type "CharacterCustomInfo Structure"))
  ;[1 1 1] Success Call API
  (`self.OnCharacterCustomGet` ParseData))

(event `self.OnFailCharacterCustomGetCallBack`
  ;[1 1 1] OnFail Call API
  (`self.OnFailCharacterCustomGet`))

(event `self.OnFailCharacterCustomCreateCallBack`
  ;[1 1 1] OnFail Call API
  (`self.OnFailCharacterCustomCreate`))

(event `self.OnCharacterCustomCreateCallBack`
  (params (ParseData :type "CharacterCustomInfo Structure"))
  ;[1 1 1] Success Call API
  (`self.OnCharacterCustomCreate` ParseData))

(event `self.OnFailCharacterCustomUpdateCallBack`
  ;[1 1 1] OnFail Call API
  (`self.OnFailCharacterCustomUpdate`))

(event `self.OnCharacterCustomUpdateCallBack`
  (params (ParseData :type "CharacterCustomInfo Structure"))
  ;[1 1 1] Success Call API
  (`self.OnCharacterCustomUpdate` (struct)))

(event `self.OnFailCharacterCustomDeleteCallBack`
  ;[1 1 1] OnFail Call API
  (`self.OnFailCharacterCustomDelete`))

(event `self.OnCharacterCustomDeleteCallBack`
  ;[1 1 1] Success Call API
  (`self.OnCharacterCustomDelete`))