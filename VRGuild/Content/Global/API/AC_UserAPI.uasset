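; AC_UserAPI is the user API component that relays results of user info requests through event dispatchers.
; It covers three queries (the user's own info, user info and member info), each with a success and a failure callback.
; Each callback calls its matching dispatcher, passing the returned data on success and nothing on failure.
; The graph only forwards results and contains no request logic.
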(event `self.OnUserOwnInfoGetCallBack`
  (params (UserInfo :type "UserInfo Structure (by ref)"))
  (`self.OnUserOwnInfoGet` UserInfo))

(event `self.OnFailUserOwnInfoGetCallBack`
  (`self.OnFailUserOwnInfoGet`))

(event `self.OnUserInfoGetCallBack`
  (params (UserInfo :type "UserInfo Structure (by ref)"))
  (`self.OnUserInfoGet` UserInfo))

(event `self.OnFailUserInfoGetCallBack`
  (`self.OnFailUserInfoGet`))

(event `self.OnFailUserMemberInfoGetCallBack`
  (`self.OnFailUserMemberInfoGet`))

(event `self.OnUserMemberInfoGetCallBack`
  (params (MemberInfo :type "UserMemberInfo Structure (by ref)"))
  (`self.OnUserMemberInfoGet` MemberInfo))