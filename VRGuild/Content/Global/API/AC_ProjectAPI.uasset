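; AC_ProjectAPI is an actor component that relays results of project API requests, covering create, get, update, detail, lists, team, comments and apply.
; Each request has a success and a failure callback event, and each forwards straight to a matching Call function, which appears to broadcast an event dispatcher.
; Success callbacks mostly pass their payload through, while only the apply failure carries an error message.
; The graph holds no request logic of its own.
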(event `self.OnProjectCreateCallBack`
  (params (ProjectInfo :type "ProjectInfo Structure (by ref)"))
  ;[1 1 1] ProjectCreate
  (`self.OnProjectCreate` ProjectInfo))

(event `self.OnFailProjectCreateCallBack`
  ;[1 1 1] ProjectCreate
  (`self.OnFailProjectCreate`))

(event `self.OnProjectGetCallBack`
  (params (ProjectInfo :type "ProjectInfo Structure (by ref)"))
  ;[1 1 1] Project Get
  (`self.OnProjectGet` ProjectInfo))

(event `self.OnFailProjectGetCallBack`
  ;[1 1 1] Project Get
  (`self.OnFailProjectGet`))

(event `self.OnProjectUpdateCallBack`
  (params (ProjectInfo :type "ProjectInfo Structure (by ref)"))
  ;[1 1 1] Update
  (`self.OnProjectUpdate` (struct)))

(event `self.OnFailProjectUpdateCallBack`
  ;[1 1 1] Update
  (`self.OnFailProjectUpdate`))

(event `self.OnProjectDetailGetCallBack`
  (params (ProjectDetail :type "ProjectWithDetail Structure (by ref)"))
  ;[1 1 1] Detail
  (`self.OnProjectDetailGet` ProjectDetail))

(event `self.OnFailProjectDetailGetCallBack`
  ;[1 1 1] Detail
  (`self.OnFailProjectDetailGet`))

(event `self.OnProjectListGetCallBack`
  (params (ParsedResponse :type "ProjectPagedResponse Structure"))
  ;[1 1 1] Detail List
  (`self.OnProjectListGet` ParsedResponse))

(event `self.OnFailProjectListGetCallBack`
  ;[1 1 1] Detail List
  (`self.OnFailProjectListGet`))

(event `self.OnProjectDetailListGetCallBack`
  (params (ParsedResponse :type "ProjectDetailPagedResponse Structure"))
  (`self.OnProjectDetailListGet` ParsedResponse))

(event `self.OnFailProjectDetailListGetCallBack`
  (`self.OnFailProjectDetailListGet`))

(event `self.OnProjectTeamListGetCallBack`
  (params (TeamList :type "ProjectTeamList Structure (by ref)"))
  ;[1 1 1] Get Team
  (`self.OnProjectTeamListGet` TeamList))

(event `self.OnFailProjectTeamListGetCallBack`
  ;[1 1 1] Get Team
  (`self.OnFailProjectTeamListGet`))

(event `self.OnProjectCommentListGetCallBack`
  (params (CommentList :type "ProjectInfo Structure (by ref)"))
  ;[1 1 1] GetComment
  (`self.OnProjectCommentListGet` CommentList))

(event `self.OnFailProjectCommentListGetCallBack`
  ;[1 1 1] GetComment
  (`self.OnFailProjectCommentListGet`))

(event `self.OnProjectApplyCallBack`
  (params (TeamList :type "ProjectTeamList Structure (by ref)"))
  ;[1 1 1] Get apply
  (`self.OnProjectApply` TeamList))

(event `self.OnFailProjectApplyCallBack`
  (params (ErrorMessage :type String))
  ;[1 1 1] Get apply
  (`self.OnFailProjectApply` ErrorMessage))