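; AC_DeveloperAPI is a component that relays results of developer-record API requests to the rest of the game.
; It covers four operations: create, get, update and get by user ID, each with success and failure callbacks.
; Each callback calls a matching event dispatcher, passing DeveloperInfo on success and nothing on failure.
; The graph holds only this pass-through; the requests themselves are not issued here.
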(event `self.OnDeveloperCreateCallBack`
  (params (DeveloperInfo :type "DevInfo Structure (by ref)"))
  ;[1 1 1] Create
  (`self.OnDevCreate` DeveloperInfo))

(event `self.OnFailDeveloperCreateCallBack`
  ;[1 1 1] Create
  (`self.OnDevCreateFail`))

(event `self.OnDeveloperGetCallBack`
  (params (DeveloperInfo :type "DevInfo Structure (by ref)"))
  ;[1 1 1] Get
  (`self.OnDevGet` DeveloperInfo))

(event `self.OnFailDeveloperGetCallBack`
  ;[1 1 1] Get
  (`self.OnDevGetFail`))

(event `self.OnDeveloperUpdateCallBack`
  (params (DeveloperInfo :type "DevInfo Structure (by ref)"))
  ;[1 1 1] Update
  (`self.OnDevUpdate` DeveloperInfo))

(event `self.OnFailDeveloperUpdateCallBack`
  ;[1 1 1] Update
  (`self.OnDevUpdateFail`))

(event `self.OnDeveloperGetByUserIdCallBack`
  (params (DeveloperInfo :type "DevInfo Structure (by ref)"))
  ;[1 1 1] Get by User Id
  (`self.OnDevGetByUserId` DeveloperInfo))

(event `self.OnFailDeveloperGetByUserIdCallBack`
  ;[1 1 1] Get by User Id
  (`self.OnDevGetByUserIdFail`))