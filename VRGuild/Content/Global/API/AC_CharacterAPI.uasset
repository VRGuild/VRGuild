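; AC_CharacterAPI is a component that relays the results of character API requests to listeners through event dispatchers.
; Callback events for create, get, update and get-by-user-ID broadcast matching success or failure dispatchers, with successes passing CharacterInfo along.
; The get-by-nickname callbacks are empty stubs marked as unused.
; The event graph only forwards results and issues no requests itself.
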(event `self.OnCharacterCreateCallBack`
  (params (CharacterInfo :type "CharacterInfo Structure (by ref)"))
  ;[1 1 1] Create Call
  (`self.OnCharacterCreate` CharacterInfo))

(event `self.OnFailCharacterCreateCallBack`
  ;[1 1 1] Create Call
  (`self.OnFailCharacterCreate`))

(event `self.OnCharacterGetCallBack`
  (params (CharacterInfo :type "CharacterInfo Structure (by ref)"))
  ;[1 1 1] Character Get
  (`self.OnCharacterGet` CharacterInfo))

(event `self.OnFailCharacterGetCallBack`
  ;[1 1 1] Character Get
  (`self.OnFailCharacterGet`))

(event `self.OnCharacterUpdateCallBack`
  (params (CharacterInfo :type "CharacterInfo Structure (by ref)"))
  ;[1 1 1] Character update Call
  (`self.OnCharacterUpdate` CharacterInfo))

(event `self.OnFailCharacterUpdateCallBack`
  ;[1 1 1] Character update Call
  (`self.OnFailCharacterUpdate`))

(event `self.OnCharacterGetByUserIdCallBack`
  (params (CharacterInfo :type "CharacterInfo Structure (by ref)"))
  ;[1 1 1] Character get by UserId
  (`self.OnCharacterGetUserId` CharacterInfo))

(event `self.OnFailCharacterGetByUserIdCallBack`
  ;[1 1 1] Character get by UserId
  (`self.OnFailCharacterGetUserId`))

(event `self.OnCharacterGetByNicknameCallBack`
  (params (CharacterInfo :type "CharacterInfo Structure (by ref)"))
  ;[1 1 1] Character Get NickName (not Use)
)

(event `self.OnFailCharacterGetByNicknameCallBack`
  ;[1 1 1] Character Get NickName (not Use)
)