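; Base player controller that hosts Login, Tile and Ether API components for making server calls.
; The OnLoginAPICall event triggers the Ether component's post call, despite its login name, while the Login and Tile post calls are left unconnected.
; Each component's callback event only prints a placeholder "Hello", so no response data is handled here.
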(event `self.OnLoginAPICall`
  (`CACEtherAPI.EtherPostCall` (`self.AC_EtherAPI`)))

(event `self.AC_LoginAPI.OnLoginAPI`
  (`KismetSystemLibrary.PrintString` "Hello"))

(event `self.AC_TileAPI.OnTileAPI`
  (`KismetSystemLibrary.PrintString` "Hello"))

(event `self.AC_EtherAPI.OnEtherAPICallBack`
  (`KismetSystemLibrary.PrintString` "Hello"))

(fn `UserConstructionScript`)