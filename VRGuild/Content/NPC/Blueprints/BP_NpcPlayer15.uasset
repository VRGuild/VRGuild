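; NPC character Blueprint with a modular body, a nameplate showing nickname and skill image, and looping idle behavior.
; The construction script fills the nameplate widget and makes head, top, bottom and hair follow the main mesh through leader pose; BeginPlay fills the nameplate again.
; A looping timer periodically plays a patting animation, then a talking one after a delay.
; Tick yaws the nameplate toward the local player's camera.
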(event `self.ReceiveBeginPlay`
  (`|ExecutionSequence`
    (:`then_0`
      (bind _aswbp_character_nickname (cast `/Game/Character/UI/WBP_Character_Nickname` (`WidgetComponent.GetWidget` (`self.Widget`))))
      (`/Game/Character/UI/WBP_Character_Nickname.SetNickname` _aswbp_character_nickname (`self.Nickname`))
      (`/Game/Character/UI/WBP_Character_Nickname.SetSkillImage` _aswbp_character_nickname (`self.NPCSkill`)))
    (:`then_1`
      (`KismetSystemLibrary.K2_SetTimerDelegate` (delegate `Play animation`) 10.0 true))))

(event `Play animation`
  (`SkeletalMeshComponent.PlayAnimation` (`self.Mesh`) "/Game/NPC/Animation/AN_npc2_Patting_UE.AN_npc2_Patting_UE" false)
  (`KismetSystemLibrary.Delay` 3.0)
  (`SkeletalMeshComponent.PlayAnimation` (`self.Mesh`) "/Game/NPC/Animation/AN_npc_Talking_UE.AN_npc_Talking_UE" false))

(event `self.ReceiveTick`
  (params (DeltaSeconds :type "Float (single-precision)"))
  (bind _returnvalue (`GameplayStatics.GetPlayerController` 0))
  (bind _widget (`self.Widget`))
  (bind (_returnvalue_roll _returnvalue_pitch) (`KismetMathLibrary.BreakRotator` (`SceneComponent.K2_GetComponentRotation` _widget)))
  (bind (_returnvalue_roll_2 _returnvalue_pitch_2 _returnvalue_yaw) (`KismetMathLibrary.BreakRotator` (`PlayerCameraManager.GetCameraRotation` (`PlayerController.PlayerCameraManager` _returnvalue))))
  (`/Engine/EditorBlueprintResources/StandardMacros.IsValid` _returnvalue
    (:`Is Valid`
      (`SceneComponent.K2_SetWorldRotation` _widget (`KismetMathLibrary.MakeRotator` _returnvalue_roll _returnvalue_pitch (- _returnvalue_yaw 180.0)) false false))))

(fn `UserConstructionScript`
  (bind _aswbp_character_nickname (cast `/Game/Character/UI/WBP_Character_Nickname` (`WidgetComponent.GetWidget` (`self.Widget`))))
  (`/Game/Character/UI/WBP_Character_Nickname.SetNickname` _aswbp_character_nickname (`self.Nickname`))
  (`/Game/Character/UI/WBP_Character_Nickname.SetSkillImage` _aswbp_character_nickname (`self.NPCSkill`))
  (`SkinnedMeshComponent.SetLeaderPoseComponent` (`self.head1`) (`self.Mesh`) false false)
  (`SkinnedMeshComponent.SetLeaderPoseComponent` (`self.Top1`) (`self.Mesh`) false false)
  (`SkinnedMeshComponent.SetLeaderPoseComponent` (`self.Bottom1`) (`self.Mesh`) false false)
  (`SkinnedMeshComponent.SetLeaderPoseComponent` (`self.Hair1`) (`self.Mesh`) false false))