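; Networked character Blueprint with camera-driven look-at angles, widget interaction and a stored voice chat name.
; Each tick on the authority, it derives pitch and yaw from the follow camera relative to the actor, limiting upward pitch and updating yaw only within a frontal arc.
; A server-to-multicast event chain shares both angles.
; Remote instances activate the widget interaction component at BeginPlay, and the interact input drives its left-click press and release.
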(event `self.ReceiveBeginPlay`
  (`/Engine/EditorBlueprintResources/ActorMacros.Switch Has Authority`
    (:`Remote`
      (`ActorComponent.Activate` (`self.WidgetInteractionComp`) false))))

(event `EnhancedInput|/Game/Global/Input/Actions/IA_Interact`
  (params (ActionValue :type Boolean) (ElapsedSeconds :type "Float (double-precision)") (TriggeredSeconds :type "Float (double-precision)") (InputAction :type "InputAction Object Reference" :default "/Game/Global/Input/Actions/IA_Interact.IA_Interact"))
  (bind _widgetinteractioncomp (`self.WidgetInteractionComp`))
  (:`Started`
    (`WidgetInteractionComponent.PressPointerKey` _widgetinteractioncomp "LeftMouseButton"))
  (:`Completed`
    (`WidgetInteractionComponent.ReleasePointerKey` _widgetinteractioncomp "LeftMouseButton")))

(event `ServerSetVoiceChatName`
  (params (VoiceChatUserName :type String))
  (set `self.VoiceChatName` VoiceChatUserName))

(event `self.ReceiveTick`
  (params (DeltaSeconds :type "Float (single-precision)"))
  (bind _pitch (.pitch (`self.K2_GetActorRotation` self)))
  (bind (_returnvalue_roll _returnvalue_pitch _returnvalue_yaw) (`KismetMathLibrary.BreakRotator` (`SceneComponent.GetSocketRotation` (`self.FollowCamera`) "None")))
  (bind _returnvalue (- _returnvalue_yaw (.yaw (`self.K2_GetActorRotation` self))))
  (bind _returnvalue_2 (- _returnvalue_pitch _pitch))
  (`|ExecutionSequence`
    (:`then_0`
      (`/Engine/EditorBlueprintResources/ActorMacros.Switch Has Authority`
        (:`Authority`
          (`|ExecutionSequence`
            (:`then_0`
              (if (< _returnvalue_2 30.0)
                (set `self.Look at Pitch` _returnvalue_2)
                (else
                  (set `self.Look at Pitch` (+ _pitch 30.0)))))
            (:`then_1`
              (if (< (`KismetMathLibrary.Abs` _returnvalue) 60.0)
                (set `self.Look at Yaw` _returnvalue :!label _label)
                (elif (< (`KismetMathLibrary.Abs` (+ _returnvalue 360.0)) 60.0)
                  (goto _label))))
            (:`then_2`
              (`self.RPCServerSend` (`self.Look at Pitch`) (`self.Look at Yaw`)))))))))

(event `RPCServerSend`
  (params (Pitch :type "Float (double-precision)") (Yaw :type "Float (double-precision)"))
  (`self.RPCMultiSendData` Pitch Yaw))

(event `RPCMultiSendData`
  (params (Pitch :type "Float (double-precision)") (Yaw :type "Float (double-precision)"))
  (set `self.Look at Pitch` Pitch)
  (set `self.Look at Yaw` Yaw))

(fn `GetVoiceChatUserName`
  (returns (VoiceChatName :type String))
  (return (`self.VoiceChatName`)))

(fn `RPCServerSendData`
  (params (Pitch1 :type "Float (double-precision)") (Yaw1 :type "Float (double-precision)")))

(fn `UserConstructionScript`)