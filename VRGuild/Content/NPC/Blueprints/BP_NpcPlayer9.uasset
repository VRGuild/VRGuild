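; NPC character Blueprint that plays a scripted, timed animation sequence when play begins.
; BeginPlay calls the parent, then plays a looping talk, a one-shot victory idle and a looping standing talk on the Mesh, separated by delays.
; The construction script makes the skeletal body, hair, top and bottom parts follow the Mesh through leader pose.
; RPCServerSendData is an empty stub, and GetVoiceChatUserName returns the stored voice chat name.
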(event `self.ReceiveBeginPlay`
  (`parent.ReceiveBeginPlay`)
  (`SkeletalMeshComponent.PlayAnimation` (`self.Mesh`) "/Game/NPC/Animation/AN_npc_Talking_UE.AN_npc_Talking_UE" true)
  (`KismetSystemLibrary.Delay` 5.0)
  (`SkeletalMeshComponent.PlayAnimation` (`self.Mesh`) "/Game/NPC/Animation/AN_npc_VictoryIdle_UE.AN_npc_VictoryIdle_UE" false)
  (`KismetSystemLibrary.Delay` 2.0)
  (`SkeletalMeshComponent.PlayAnimation` (`self.Mesh`) "/Game/NPC/Animation/AN_npc_StandTalking_UE.AN_npc_StandTalking_UE" true))

(fn `GetVoiceChatUserName`
  (returns (VoiceChatName :type String))
  (return (`self.VoiceChatName`)))

(fn `RPCServerSendData`
  (params (Pitch1 :type "Float (double-precision)") (Yaw1 :type "Float (double-precision)")))

(fn `UserConstructionScript`
  (`SkinnedMeshComponent.SetLeaderPoseComponent` (`self.SkeletalMesh_0`) (`self.Mesh`) false false)
  (`SkinnedMeshComponent.SetLeaderPoseComponent` (`self.hair_0`) (`self.Mesh`) false false)
  (`SkinnedMeshComponent.SetLeaderPoseComponent` (`self.top_0`) (`self.Mesh`) false false)
  (`SkinnedMeshComponent.SetLeaderPoseComponent` (`self.bottom_0`) (`self.Mesh`) false false))