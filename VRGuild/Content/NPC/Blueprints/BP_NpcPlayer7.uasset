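; BP_NpcPlayer7 is a seated NPC that periodically plays a clapping animation.
; The construction script makes its modular skeletal parts, including top, bottom and hair, follow the main Mesh through leader pose.
; On BeginPlay a looping ten-second timer plays the one-shot sitting clap animation on the Mesh.
; It also has an empty RPCServerSendData function and a getter returning its voice chat name.
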(event `self.ReceiveBeginPlay`
  (`parent.ReceiveBeginPlay`)
  (`KismetSystemLibrary.K2_SetTimerDelegate` (delegate `PlayClapAnim`) 10.0 true))

(event `PlayClapAnim`
  (`SkeletalMeshComponent.PlayAnimation` (`self.Mesh`) "/Game/NPC/Animation/AN_npc_SittingClap_UE.AN_npc_SittingClap_UE" false))

(fn `GetVoiceChatUserName`
  (returns (VoiceChatName :type String))
  (return (`self.VoiceChatName`)))

(fn `RPCServerSendData`
  (params (Pitch1 :type "Float (double-precision)") (Yaw1 :type "Float (double-precision)")))

(fn `UserConstructionScript`
  (`SkinnedMeshComponent.SetLeaderPoseComponent` (`self.SkeletalMesh_0`) (`self.Mesh`) false false)
  (`SkinnedMeshComponent.SetLeaderPoseComponent` (`self.top_0`) (`self.Mesh`) false false)
  (`SkinnedMeshComponent.SetLeaderPoseComponent` (`self.bottom_0`) (`self.Mesh`) false false)
  (`SkinnedMeshComponent.SetLeaderPoseComponent` (`self.hair_0`) (`self.Mesh`) false false))