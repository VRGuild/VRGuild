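; Base guild room NPC, built from modular mesh parts with an overhead widget showing its nickname and skill image.
; The construction script makes head, hair, top and bottom follow the body's pose through leader pose components.
; BeginPlay pushes the nickname and NPC skill into the nickname widget.
; Tick turns that widget toward the local camera, only on the Remote (non-authority) branch.
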(event `self.ReceiveBeginPlay`
  (`self.SetNpcNickName`))

(event `self.ReceiveTick`
  (params (DeltaSeconds :type "Float (single-precision)"))
  (`/Engine/EditorBlueprintResources/ActorMacros.Switch Has Authority`
    (:`Remote`
      (`SceneComponent.K2_SetWorldRotation` (`self.Nicknamewidget`) (`KismetMathLibrary.FindLookAtRotation` (`SceneComponent.K2_GetComponentLocation` (`self.Nicknamewidget`)) (`SceneComponent.K2_GetComponentLocation` (`PlayerCameraManager.TransformComponent` (`GameplayStatics.GetPlayerCameraManager` 0)))) false false))))

(event `SetNpcNickName`
  (bind _aswbp_character_nickname (cast `/Game/Character/UI/WBP_Character_Nickname` (`WidgetComponent.GetWidget` (`self.Nicknamewidget`))))
  (`/Game/Character/UI/WBP_Character_Nickname.SetNickname` _aswbp_character_nickname (`self.Nickname`))
  (`/Game/Character/UI/WBP_Character_Nickname.SetSkillImage` _aswbp_character_nickname (`self.NPCSkill`)))

(fn `UserConstructionScript`
  (`SkinnedMeshComponent.SetLeaderPoseComponent` (`self.Head`) (`self.Body`) false false)
  (`SkinnedMeshComponent.SetLeaderPoseComponent` (`self.Hair`) (`self.Body`) false false)
  (`SkinnedMeshComponent.SetLeaderPoseComponent` (`self.Top`) (`self.Body`) false false)
  (`SkinnedMeshComponent.SetLeaderPoseComponent` (`self.Bottom`) (`self.Body`) false false))