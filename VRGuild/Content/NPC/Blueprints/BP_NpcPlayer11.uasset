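; BP_NpcPlayer11 is a character Blueprint, named as an NPC player, with a modular body and a stored voice chat name.
; The construction script makes the SkeletalMesh, Hair, Top and Bottom components follow Mesh through leader pose.
; ServerSetVoiceChatName stores the name, and GetVoiceChatUserName returns it.
; BeginPlay, Tick, the interact input and RPCServerSendData are empty stubs.
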(event `self.ReceiveBeginPlay`)

(event `EnhancedInput|/Game/Global/Input/Actions/IA_Interact`
  (params (ActionValue :type Boolean) (ElapsedSeconds :type "Float (double-precision)") (TriggeredSeconds :type "Float (double-precision)") (InputAction :type "InputAction Object Reference" :default "/Game/Global/Input/Actions/IA_Interact.IA_Interact")))

(event `ServerSetVoiceChatName`
  (params (VoiceChatUserName :type String))
  (set `self.VoiceChatName` VoiceChatUserName))

(event `self.ReceiveTick`
  (params (DeltaSeconds :type "Float (single-precision)")))

(fn `GetVoiceChatUserName`
  (returns (VoiceChatName :type String))
  (return (`self.VoiceChatName`)))

(fn `RPCServerSendData`
  (params (Pitch1 :type "Float (double-precision)") (Yaw1 :type "Float (double-precision)")))

(fn `UserConstructionScript`
  (`SkinnedMeshComponent.SetLeaderPoseComponent` (`self.SkeletalMesh`) (`self.Mesh`) false false)
  (`SkinnedMeshComponent.SetLeaderPoseComponent` (`self.hair`) (`self.Mesh`) false false)
  (`SkinnedMeshComponent.SetLeaderPoseComponent` (`self.top`) (`self.Mesh`) false false)
  (`SkinnedMeshComponent.SetLeaderPoseComponent` (`self.bottom`) (`self.Mesh`) false false))