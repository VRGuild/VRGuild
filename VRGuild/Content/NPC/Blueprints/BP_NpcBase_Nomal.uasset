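; Base NPC with a looping animation, voice audio and an overhead nickname widget showing its name and skill image.
; The construction script makes the modular body, hair and clothing meshes follow the main Mesh through leader pose.
; Voice starts on BeginPlay or sphere overlap, guarded by a playing flag, and replays when finished.
; Every tick, only without authority, the nickname widget rotates toward the player camera.
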(event `self.ReceiveBeginPlay`
  (`self.PlayNpcSound`)
  (`self.PlayNpcAnimation`)
  (`self.SetNpcNickName`))

(event `self.ReceiveTick`
  (params (DeltaSeconds :type "Float (single-precision)"))
  (`self.Update`))

(event `Update`
  ;[1 1 1] Called on tick
  (`/Engine/EditorBlueprintResources/ActorMacros.Switch Has Authority`
    (:`Remote`
      (`SceneComponent.K2_SetWorldRotation` (`self.Nicknamewidget`) (`KismetMathLibrary.FindLookAtRotation` (`SceneComponent.K2_GetComponentLocation` (`self.Nicknamewidget`)) (`SceneComponent.K2_GetComponentLocation` (`PlayerCameraManager.TransformComponent` (`GameplayStatics.GetPlayerCameraManager` 0)))) false false))))

(event `self.Audio.OnAudioFinished`
  (set `self.bissound` false)
  (`AudioComponent.Play` (`self.Audio`) 0.0))

(event `PlayNpcSound`
  (bind _audio (`self.Audio`))
  (bind _npcvoicesound (`self.NPCVoiceSound`))
  (if (not (`self.bissound`))
    (`/Engine/EditorBlueprintResources/StandardMacros.IsValid` _npcvoicesound
      (:`Is Valid`
        (`AudioComponent.SetSound` _audio _npcvoicesound)
        (`ActorComponent.SetAutoActivate` _audio true)
        (`AudioComponent.Play` _audio 0.0)
        (set `self.bissound` true))
      (:`Is Not Valid`
        (set `self.bissound` false)))))

(event `PlayNpcAnimation`
  (bind _npcanimation (`self.NPCAnimation`))
  (`/Engine/EditorBlueprintResources/StandardMacros.IsValid` _npcanimation
    (:`Is Valid`
      (`SkeletalMeshComponent.PlayAnimation` (`self.Mesh`) _npcanimation true))))

(event `SetNpcNickName`
  (bind _aswbp_character_nickname (cast `/Game/Character/UI/WBP_Character_Nickname` (`WidgetComponent.GetWidget` (`self.Nicknamewidget`))))
  (`/Game/Character/UI/WBP_Character_Nickname.SetNickname` _aswbp_character_nickname (`self.Nickname`))
  (`/Game/Character/UI/WBP_Character_Nickname.SetSkillImage` _aswbp_character_nickname (`self.NPCSkill`)))

(event `self.Sphere.OnComponentBeginOverlap`
  (params (OverlappedComponent :type "PrimitiveComponent Object Reference") (OtherActor :type "Actor Object Reference") (OtherComp :type "PrimitiveComponent Object Reference") (OtherBodyIndex :type Integer) (bFromSweep :type Boolean) (SweepResult :type "HitResult Structure (by ref)"))
  (`self.PlayNpcSound`))

(fn `UserConstructionScript`
  (`SkinnedMeshComponent.SetLeaderPoseComponent` (`self.SkeletalMesh`) (`self.Mesh`) false false)
  (`SkinnedMeshComponent.SetLeaderPoseComponent` (`self.Hair`) (`self.Mesh`) false false)
  (`SkinnedMeshComponent.SetLeaderPoseComponent` (`self.Top`) (`self.Mesh`) false false)
  (`SkinnedMeshComponent.SetLeaderPoseComponent` (`self.Bottom`) (`self.Mesh`) false false))