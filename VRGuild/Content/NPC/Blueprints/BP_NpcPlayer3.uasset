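; NPC character Blueprint that displays a nickname and skill image on a widget and stores a voice chat user name.
; The construction script makes the modular body, hair, top and bottom meshes follow the main Mesh through leader pose.
; Both construction and BeginPlay call SetNpcNickName, then push Nickname and NPCSkill into the WBP_Character_Nickname widget.
; ServerSetVoiceChatName sets the voice name returned by GetVoiceChatUserName, while Tick and RPCServerSendData are empty.
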(event `self.ReceiveBeginPlay`
  (`self.SetNpcNickName`)
  (bind _aswbp_character_nickname (cast `/Game/Character/UI/WBP_Character_Nickname` (`WidgetComponent.GetWidget` (`self.Widget`))))
  (`/Game/Character/UI/WBP_Character_Nickname.SetNickname` _aswbp_character_nickname (`self.Nickname`))
  (`/Game/Character/UI/WBP_Character_Nickname.SetSkillImage` _aswbp_character_nickname (`self.NPCSkill`)))

(event `ServerSetVoiceChatName`
  (params (VoiceChatUserName :type String))
  (set `self.VoiceChatName` VoiceChatUserName))

(event `self.ReceiveTick`
  (params (DeltaSeconds :type "Float (single-precision)")))

(fn `GetVoiceChatUserName`
  (returns (VoiceChatName :type String))
  (return (`self.VoiceChatName`)))

(fn `RPCServerSendData`
  (params (Pitch1 :type "Float (double-precision)") (Yaw1 :type "Float (double-precision)")))

(fn `UserConstructionScript`
  (`SkinnedMeshComponent.SetLeaderPoseComponent` (`self.SkeletalMesh_0`) (`self.Mesh`) false false)
  (`SkinnedMeshComponent.SetLeaderPoseComponent` (`self.hair_0`) (`self.Mesh`) false false)
  (`SkinnedMeshComponent.SetLeaderPoseComponent` (`self.top_0`) (`self.Mesh`) false false)
  (`SkinnedMeshComponent.SetLeaderPoseComponent` (`self.bottom_0`) (`self.Mesh`) false false)
  (`self.SetNpcNickName`)
  (bind _aswbp_character_nickname (cast `/Game/Character/UI/WBP_Character_Nickname` (`WidgetComponent.GetWidget` (`self.Widget`))))
  (`/Game/Character/UI/WBP_Character_Nickname.SetNickname` _aswbp_character_nickname (`self.Nickname`))
  (`/Game/Character/UI/WBP_Character_Nickname.SetSkillImage` _aswbp_character_nickname (`self.NPCSkill`)))