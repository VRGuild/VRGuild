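; BP_NpcPlayer14 is an NPC Blueprint, apparently one of a numbered set, that assembles a modular character from separate skeletal mesh parts.
; Its construction script sets Mesh as the leader pose component for the Bottom, Top, SkeletalMesh and Hair parts.
; The parts follow the bone transforms of Mesh, so one animated skeleton drives the whole outfit.
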(fn `UserConstructionScript`
  (`SkinnedMeshComponent.SetLeaderPoseComponent` (`self.Bottom`) (`self.Mesh`) false false)
  (`SkinnedMeshComponent.SetLeaderPoseComponent` (`self.Top`) (`self.Mesh`) false false)
  (`SkinnedMeshComponent.SetLeaderPoseComponent` (`self.SkeletalMesh`) (`self.Mesh`) false false)
  (`SkinnedMeshComponent.SetLeaderPoseComponent` (`self.Hair`) (`self.Mesh`) false false))