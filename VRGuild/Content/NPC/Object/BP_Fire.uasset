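; BP_Fire is an NPC-folder object, apparently a fire, that plays a sound when something begins overlapping its sphere.
; The overlap calls PlayNpcSound, which checks the Bissound flag and a validity test before playing the Audio component and setting the flag.
; When the audio finishes, the flag clears and playback restarts immediately, looping the sound with the flag left false.
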(event `self.Sphere.OnComponentBeginOverlap`
  (params (OverlappedComponent :type "PrimitiveComponent Object Reference") (OtherActor :type "Actor Object Reference") (OtherComp :type "PrimitiveComponent Object Reference") (OtherBodyIndex :type Integer) (bFromSweep :type Boolean) (SweepResult :type "HitResult Structure (by ref)"))
  (`self.PlayNpcSound`))

(event `self.Audio.OnAudioFinished`
  (set `self.bissound` false)
  (`AudioComponent.Play` (`self.Audio`) 0.0))

(event `PlayNpcSound`
  (if (not (`self.bissound`))
    (`/Engine/EditorBlueprintResources/StandardMacros.IsValid` null
      (:`Is Valid`
        (`AudioComponent.Play` (`self.Audio`) 0.0)
        (set `self.bissound` true))
      (:`Is Not Valid`
        (set `self.bissound` false)))))

(fn `UserConstructionScript`)