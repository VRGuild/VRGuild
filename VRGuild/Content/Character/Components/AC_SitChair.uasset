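; AC_SitChair is a character component that lets BP_CharacterHallPlayer sit on a nearby Sitting_chair.
; The player's SitCheckCollision overlap stores the latest chair, never clearing it on exit.
; Pressing Q, if the chair allows sitting, starts the DANCE montage locally and calls ServerMoveTo with a spot above SitArrow and offset chair yaw.
; ServerMoveTo relays to MultiMoveTo, which debug-prints yaw and eases the root component there.
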(event `ServerMoveTo`
  (params (NewParam :type "SceneComponent Object Reference") (Location :type "Vector Structure") (Rotation :type "Rotator Structure"))
  (`self.MultiMoveTo` NewParam Location (`KismetMathLibrary.MakeRotator` 0.0 0.0 Rotation_Yaw)))

(event `MultiMoveTo`
  (params (NewParam :type "SceneComponent Object Reference") (Location :type "Vector Structure") (Rotation :type "Rotator Structure"))
  (`KismetSystemLibrary.PrintString` (`KismetStringLibrary.Conv_DoubleToString` Rotation_Yaw) true true (struct :`G` 0.66 :`B` 1.0 :`A` 1.0) 5.0)
  (`KismetSystemLibrary.MoveComponentTo` NewParam Location (`KismetMathLibrary.MakeRotator` 0.0 0.0 Rotation_Yaw) true true))

(event `Key|Q`
  (params (Key :type "Key Structure"))
  (bind _near_chair (`self.near chair`))
  (bind _as_bp_character_hall_player (`self.As BP Character Hall Player`))
  (bind (_returnvalue_roll _returnvalue_pitch _returnvalue_yaw) (`KismetMathLibrary.BreakRotator` (`Actor.K2_GetActorRotation` _near_chair)))
  (:`Pressed`
    (if (`/Game/TileSystem/Mesh/test/Sitting_chair.CanSit` (`self.near chair`))
      (`/Game/Character/Player/Animation/montage/AC_AnimMontage.BP_StartAnimMontage` (`/Game/Hall/Blueprints/BP_CharacterHallPlayer.AC_AnimMontage` (`self.As BP Character Hall Player`)) "DANCE")
      (`self.ServerMoveTo` (`Actor.RootComponent` _as_bp_character_hall_player) (+ (`KismetMathLibrary.MakeVector` 0.0 0.0 (`CapsuleComponent.CapsuleHalfHeight` (`Character.CapsuleComponent` _as_bp_character_hall_player))) (`SceneComponent.K2_GetComponentLocation` (`/Game/TileSystem/Mesh/test/Sitting_chair.Sit arrow` _near_chair))) (`KismetMathLibrary.MakeRotator` 0.0 0.0 (- _returnvalue_yaw 60.0))))))

(event `self.ReceiveBeginPlay`
  (bind _output_get (set `self.Owner` (`self.GetOwner`)))
  (bind _asbp_character_hall_player (cast `/Game/Hall/Blueprints/BP_CharacterHallPlayer` _output_get))
  (set `self.As BP Character Hall Player` _asbp_character_hall_player)
  (add `PrimitiveComponent.OnComponentBeginOverlap` (`/Game/Hall/Blueprints/BP_CharacterHallPlayer.SitCheckCollision` (`self.As BP Character Hall Player`)) (delegate `OnComponentBeginOverlap_Event`)))

(event `OnComponentBeginOverlap_Event`
  (params (OverlappedComponent :type "PrimitiveComponent Object Reference") (OtherActor :type "Actor Object Reference") (OtherComp :type "PrimitiveComponent Object Reference") (OtherBodyIndex :type Integer) (bFromSweep :type Boolean) (SweepResult :type "HitResult Structure (by ref)"))
  (bind _assitting_chair (cast `/Game/TileSystem/Mesh/test/Sitting_chair` OtherActor))
  (set `self.near chair` _assitting_chair))