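; Player controller for the character customization stage that handles post-login data loading before connecting the player to the server.
; Remote clients open a loading widget, and the login event fetches user info through API components, then checks character and developer data.
; Saved customization is applied through pawn components, or the customization setup starts when data is missing.
; User, character and developer flags each retry TryServerTravel, which connects once all three are true.
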(event `self.ReceiveBeginPlay`
  ;[1 1 1] Show loading Page
  (`/Engine/EditorBlueprintResources/ActorMacros.Switch Has Authority`
    (:`Remote`
      (bind _returnvalue (`|CreateWidget` "/Game/Global/UI/Loading/WBP_LoadingCustomData.WBP_LoadingCustomData_C"))
      (`UserWidget.AddToViewport` _returnvalue 0)
      (`WidgetBlueprintLibrary.SetInputMode_UIOnlyEx` self _returnvalue))))

(event `self.OnLoginAPICall`
  ;[1 1 1] Epic Login Successed
  (bind _returnvalue (`AddComponent|NODE_AddAC_UserAPI-0`))
  (add `/Game/Global/API/AC_UserAPI.OnUserOwnInfoGet` _returnvalue (`|CreateDelegate` :!event `HasUserID`))
  (add `/Game/Global/API/AC_UserAPI.OnFailUserOwnInfoGet` _returnvalue (`|CreateDelegate` :!event `FailGetUserId`))
  (`CACUserAPI.UserOwnInfoGetCall` _returnvalue))

(event `HasUserID`
  (params (UserInfo :type "UserInfo Structure"))
  ;[1 1 1] Epic Login Successed
  (bind _asgi_base (cast `/Game/Global/GI_Base` (`GameplayStatics.GetGameInstance`)))
  (set `CGIGameInstance.UserId` (`.userId` (break `UserInfo` UserInfo)) _asgi_base)
  (`self.CheckHasCharacter`)
  (`self.Check Dev Info` UserInfo)
  (`self.UserIdUpdate` true))

(event `FailGetUserId`
  ;[1 1 1] Epic Login Successed
  (`KismetSystemLibrary.PrintString` "SomeThing Wrong in UserAPI")
  (`self.StartCharacterCustom`))

(event `StartCharacterCustom`
  (bind _returnvalue (`GameplayStatics.GetPlayerPawn` 0))
  ;[1 0 0] 중간 단계 API에서 결와에 대한 call back으로만들어 주세요
  ;[1 1 1] Custom Character Info Is Empty
  (`AddComponent|NODE_AddAC_CustomHead-1` :`self` _returnvalue)
  (`AddComponent|NODE_AddAC_CustomBody-0` :`self` _returnvalue)
  (`AddComponent|NODE_AddAC_CustomLower-0` :`self` _returnvalue)
  ;;[1 1 1] Create Widget
  (bind _returnvalue_2 (`AddComponent|NODE_AddAC_CustomInteraction-0` :`self` _returnvalue))
  (`CACCustomInteraction.Init` _returnvalue_2 false))

(event `CheckHasCharacter`
  ;[1 1 1] BackEnd Login Successed
  ;;[1 1 1] API Info
  (bind _returnvalue (`AddComponent|NODE_AddAC_CharacterAPI-0` :`self` (`GameplayStatics.GetPlayerPawn` 0)))
  (add `/Game/Global/API/AC_CharacterAPI.OnCharacterGet` _returnvalue (`|CreateDelegate` :!event `SkipCharacterCustom`))
  (add `/Game/Global/API/AC_CharacterAPI.OnFailCharacterGet` _returnvalue (`|CreateDelegate` :!event `StartCharacterCustom`))
  (`CACCharacterAPI.CharacterGetCall` _returnvalue))

(event `SkipCharacterCustom`
  (params (`Chracter Custom Data` :type "CharacterInfo Structure"))
  ;[1 0 0] 중간 단계 API에서 결와에 대한 call back으로만들어 주세요
  (`|ExecutionSequence`
    (:`then_0`
      ;[1 1 1] Character에 대한 정보가 있습니다.
      (`KismetArrayLibrary.Array_Clear` (`self.CustomArray`))
      (for _array_element (`.customList` (break `CharacterInfo` `Chracter Custom Data`))
        (`KismetArrayLibrary.Array_Add` (`self.CustomArray`) (`.customIndex` (break `CustomInfo` _array_element))))
      ;;[1 1 1] 데이터에 대한 설정이 필요합니다.
      (bind _returnvalue (`AddComponent|NODE_AddAC_CustomInteraction-1` :`self` (`GameplayStatics.GetPlayerPawn` 0)))
      (`CACCustomInteraction.Init` _returnvalue true)
      (`CACCustomInteraction.SaveCustomSelections` _returnvalue (`self.CustomArray`)))
    (:`then_1`
      (`self.CustomCharacterUpdate` true))))

(event `OnDevGet_Event`
  (params (DevInfo :type "DevInfo Structure"))
  ;[1 1 1] Without User Id
  (`|ExecutionSequence`
    (:`then_0`
      (`CGIGameInstance.SetMainSkillCategory` (cast `/Game/Global/GI_Base` (`GameplayStatics.GetGameInstance`) :!pure true) (`|GetArrayItem` (`.skillCategoryList` (break `DevInfo` DevInfo)))))
    (:`then_1`
      (`self.DevInfoUpdate` true))))

(event `OnDevGetFail_Event`
  ;[1 1 1] Without User Id
  (`KismetSystemLibrary.PrintString` "Failed to get Dev info!" true true (struct :`R` 1.0 :`B` 0.007974 :`A` 1.0) 5.0))

(event `Check Dev Info`
  (params (UserInfo :type "UserInfo Structure"))
  (bind _userid (break `UserInfo` UserInfo))
  (bind _returnvalue (`AddComponent|NODE_AddAC_DeveloperAPI-0`))
  (if (== _userid 0)
    (`|ExecutionSequence`
      (:`then_0`
        (add `/Game/Global/API/AC_DeveloperAPI.OnDevGet` _returnvalue (`|CreateDelegate` :!event `OnDevGet_Event`)))
      (:`then_1`
        (add `/Game/Global/API/AC_DeveloperAPI.OnDevGetFail` _returnvalue (`|CreateDelegate` :!event `OnDevGetFail_Event`)))
      (:`then_2`
        (`CACDeveloperAPI.DeveloperGetCall` _returnvalue)))
    (else
      (`|ExecutionSequence`
        (:`then_0`
          (add `/Game/Global/API/AC_DeveloperAPI.OnDevGetByUserId` _returnvalue (`|CreateDelegate` :!event `Dev Get by User Id`)))
        (:`then_1`
          (add `/Game/Global/API/AC_DeveloperAPI.OnDevGetByUserIdFail` _returnvalue (`|CreateDelegate` :!event `Dev Get by User Id Fail`)))
        (:`then_2`
          (`CACDeveloperAPI.DeveloperGetByUserIdCall` _returnvalue (`KismetStringLibrary.Conv_IntToString` (`KismetMathLibrary.Conv_Int64ToInt` _userid))))))))

(event `Dev Get by User Id`
  (params (DevInfo :type "DevInfo Structure"))
  ;[1 1 1] With User Id
  (`|ExecutionSequence`
    (:`then_0`
      (`CGIGameInstance.SetMainSkillCategory` (cast `/Game/Global/GI_Base` (`GameplayStatics.GetGameInstance`) :!pure true) (`|GetArrayItem` (`.skillCategoryList` (break `DevInfo` DevInfo)))))
    (:`then_1`
      (`self.DevInfoUpdate` true))))

(event `Dev Get by User Id Fail`
  ;[1 1 1] With User Id
  (`KismetSystemLibrary.PrintString` "Failed to get Dev info with User Id!" true true (struct :`R` 1.0 :`B` 0.007974 :`A` 1.0) 5.0))

(fn `CustomCharacterUpdate`
  (params (Has :type Boolean))
  (set `self.bHasCustomCharacter` Has)
  (`self.TryServerTravel`))

(fn `DevInfoUpdate`
  (params (Has :type Boolean))
  (set `self.bHasDevInfo` Has)
  (`self.TryServerTravel`))

(fn `TryServerTravel`
  (bind _bhasuserid (`self.bHasUserId`))
  (bind _bhascustomcharacter (`self.bHasCustomCharacter`))
  (bind _bhasdevinfo (`self.bHasDevInfo`))
  (`KismetSystemLibrary.PrintString` (`KismetStringLibrary.Concat_StrStr` "Has User Id: " (`KismetStringLibrary.Conv_BoolToString` _bhasuserid) ", Has Custom Character: " (`KismetStringLibrary.Conv_BoolToString` _bhascustomcharacter) ", Has Dev Info: " (`KismetStringLibrary.Conv_BoolToString` _bhasdevinfo)))
  (if (and _bhasuserid _bhascustomcharacter _bhasdevinfo)
    (`self.ConnectToServer`)))

(fn `UserConstructionScript`)

(fn `UserIdUpdate`
  (params (bHas :type Boolean))
  (set `self.bHasUserId` bHas)
  (`self.TryServerTravel`))