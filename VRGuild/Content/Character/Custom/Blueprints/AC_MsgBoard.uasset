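; Actor component that shows a floating board with nickname and main skill above non-locally controlled third-person characters.
; On BeginPlay it creates a widget component on the owner and fills it with a character nickname widget.
; Init stores the local character, Update turns the board to face that actor, and SetHover passes custom data to the widget.
; Visibility countdown and input-mode logic is left unconnected.
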(event `self.ReceiveBeginPlay`
  (bind _returnvalue (`self.GetOwner`))
  (`Actor.EnableInput` _returnvalue (`GameplayStatics.GetPlayerController` 0))
  (bind _output_get (set `self.Owner` _returnvalue))
  (bind _astp_third_person_character (cast `TP_ThirdPersonCharacter` _output_get))
  (if (not (`Pawn.IsLocallyControlled` _astp_third_person_character))
    (bind _returnvalue_2 (`|AddComponentByClass` _astp_third_person_character "/Script/UMG.WidgetComponent" false (`KismetMathLibrary.MakeTransform` (0.0 0.0 75.0))))
    (set `self.WidgetComp` _returnvalue_2)
    (bind _returnvalue_3 (`|CreateWidget` "/Game/Character/UI/WBP_Character_Nickname.WBP_Character_Nickname_C" (`GameplayStatics.GetPlayerController` 0)))
    (`WidgetComponent.SetWidget` _returnvalue_2 _returnvalue_3)
    (set `self.WidgetMsgBoard` _returnvalue_3)))

(event `Update`
  ;[1 1 1] Called on tick
  (bind _locallycontrolled (`self.LocallyControlled`)
    (:`then`
      (`SceneComponent.K2_SetWorldRotation` (`self.WidgetComp`) (`KismetMathLibrary.FindLookAtRotation` (`SceneComponent.K2_GetComponentLocation` (`self.WidgetComp`)) (`Actor.K2_GetActorLocation` _locallycontrolled)) false false))
    (:`else`)))

(event `Init`
  (params (LocallyControlled :type "Character Object Reference"))
  (set `self.LocallyControlled` LocallyControlled)
  (`KismetSystemLibrary.PrintString` "LocallyControlled: Hover Init"))

(fn `SetHover`
  (params (CustomData :type "CharacterCustomData Structure"))
  (bind (_selections _pixels _nickname _mainskill) (break `CharacterCustomData` CustomData))
  (`|ExecutionSequence`
    (:`then_0`
      (`self.SetUsername` _nickname))
    (:`then_1`
      (`self.SetMainSkill` _mainskill))))

(fn `SetMainSkill`
  (params (SkillCategory :type "SkillCategoryInfo Structure"))
  (`/Game/Character/UI/WBP_Character_Nickname.SetMainSkill` (`self.WidgetMsgBoard`) SkillCategory))

(fn `SetUsername`
  (params (Username :type String))
  (`/Game/Character/UI/WBP_Character_Nickname.SetNickname` (`self.WidgetMsgBoard`) Username))