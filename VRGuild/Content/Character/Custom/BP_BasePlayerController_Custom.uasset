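; Player controller for character customization that starts on a loading screen and handles the Epic login step.
; BeginPlay shows WBP_Loading with UI-only input.
; OnLoginAPICall adds a login API component to the pawn, requests Epic login info, then immediately adds head, body, lower and interaction customization components.
; The OnLoginInfoAPI callback is an empty stub, so setup does not wait for the response.
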(event `self.ReceiveBeginPlay`
  (bind _returnvalue (`|CreateWidget` "/Game/Global/UI/Loading/WBP_Loading.WBP_Loading_C"))
  (`UserWidget.AddToViewport` _returnvalue 0)
  (`WidgetBlueprintLibrary.SetInputMode_UIOnlyEx` self _returnvalue))

(event `self.OnLoginAPICall`
  (bind _returnvalue (`GameplayStatics.GetPlayerPawn` 0))
  ;[1 1 1] Epic Login Successed
  (bind _returnvalue_2 (`AddComponent|NODE_AddAC_LoginAPI-0` :`self` (`GameplayStatics.GetPlayerPawn` 0)))
  (bind _output_get (set `self.LoginAPI` _returnvalue_2))
  (`CACLoginAPI.EpicLoginInfoGetCall` _output_get)
  ;[1 1 1] Custom Character Info
  (`AddComponent|NODE_AddAC_CustomHead-1` :`self` _returnvalue)
  (`AddComponent|NODE_AddAC_CustomBody-0` :`self` _returnvalue)
  (`AddComponent|NODE_AddAC_CustomLower-0` :`self` _returnvalue)
  ;;[1 1 1] Create Widget
  (`AddComponent|NODE_AddAC_CustomInteraction-0` :`self` _returnvalue))

(event `self.LoginAPI.OnLoginInfoAPI`
  ;[1 0 0] 중간 단계 API에서 결와에 대한 call back으로만들어 주세요
)

(fn `UserConstructionScript`)